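; Character Blueprint that displays equipped gear as separate skeletal mesh components, one per equipment slot.
; Each slot's mesh variable has an OnRep function that updates its component, replicating appearance changes to clients.
; Armor, clothing and accessory slots follow the body Mesh through master pose.
; Rings and hand items attach to sockets named in LocalEquipmentSockets, snapping to them except the right ring, which keeps its relative transform.
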(fn `OnRep_AccessoryMesh`
  (`SkinnedMeshComponent.SetSkinnedAssetAndUpdate` (`self.Accessory`) (`self.AccessoryMesh`) true)
  (`SkinnedMeshComponent.SetLeaderPoseComponent` (`self.Accessory`) (`self.Mesh`)))

(fn `OnRep_BackMesh`
  (`SkinnedMeshComponent.SetSkinnedAssetAndUpdate` (`self.Back`) (`self.BackMesh`) true)
  (`SkinnedMeshComponent.SetLeaderPoseComponent` (`self.Back`) (`self.Mesh`)))

(fn `OnRep_ChestMesh`
  (`SkinnedMeshComponent.SetSkinnedAssetAndUpdate` (`self.Chest`) (`self.ChestMesh`) true)
  (`SkinnedMeshComponent.SetLeaderPoseComponent` (`self.Chest`) (`self.Mesh`)))

(fn `OnRep_FeetMesh`
  (`SkinnedMeshComponent.SetSkinnedAssetAndUpdate` (`self.Feet`) (`self.FeetMesh`) true)
  (`SkinnedMeshComponent.SetLeaderPoseComponent` (`self.Feet`) (`self.Mesh`)))

(fn `OnRep_HandsMesh`
  (`SkinnedMeshComponent.SetSkinnedAssetAndUpdate` (`self.Hands`) (`self.HandsMesh`) true)
  (`SkinnedMeshComponent.SetLeaderPoseComponent` (`self.Hands`) (`self.Mesh`)))

(fn `OnRep_HeadMesh`
  (`SkinnedMeshComponent.SetSkinnedAssetAndUpdate` (`self.Head`) (`self.HeadMesh`) true)
  (`SkinnedMeshComponent.SetLeaderPoseComponent` (`self.Head`) (`self.Mesh`)))

(fn `OnRep_LeftRingMesh`
  (locals (LocalEquipmentSockets :type "/Game/InventorySystem/Blueprints/Inventory/EquipmentSockets Structure" :default (struct :`RightRing` "RightRing" :`LeftRing` "LeftRing" :`Main-Hand` "MainHand" :`Off-Hand` "OffHand")))
  (`SkinnedMeshComponent.SetSkinnedAssetAndUpdate` (`self.LeftRing`) (`self.LeftRingMesh`) true)
  (`SceneComponent.K2_AttachToComponent` (`self.LeftRing`) (`self.Mesh`) (`.LeftRing_10_66512035469F61C34EC98F90E4F97407` (break `/Game/InventorySystem/Blueprints/Inventory/EquipmentSockets` (`local.LocalEquipmentSockets`))) "SnapToTarget" "SnapToTarget" "SnapToTarget" true))

(fn `OnRep_LegsMesh`
  (`SkinnedMeshComponent.SetSkinnedAssetAndUpdate` (`self.Legs`) (`self.LegsMesh`) true)
  (`SkinnedMeshComponent.SetLeaderPoseComponent` (`self.Legs`) (`self.Mesh`)))

(fn `OnRep_MainHandMesh`
  (locals (LocalEquipmentSockets :type "/Game/InventorySystem/Blueprints/Inventory/EquipmentSockets Structure" :default (struct :`RightRing` "RightRing" :`LeftRing` "LeftRing" :`Main-Hand` "MainHand" :`Off-Hand` "OffHand")))
  (`SkinnedMeshComponent.SetSkinnedAssetAndUpdate` (`self.MainHand`) (`self.MainHandMesh`) true)
  (`SceneComponent.K2_AttachToComponent` (`self.MainHand`) (`self.Mesh`) (`.Main-Hand_14_8A558B7C43EA00D3972964BA4E935F53` (break `/Game/InventorySystem/Blueprints/Inventory/EquipmentSockets` (`local.LocalEquipmentSockets`))) "SnapToTarget" "SnapToTarget" "SnapToTarget" true))

(fn `OnRep_OffHandMesh`
  (locals (LocalEquipmentSockets :type "/Game/InventorySystem/Blueprints/Inventory/EquipmentSockets Structure" :default (struct :`RightRing` "RightRing" :`LeftRing` "LeftRing" :`Main-Hand` "MainHand" :`Off-Hand` "OffHand")))
  (`SkinnedMeshComponent.SetSkinnedAssetAndUpdate` (`self.OffHand`) (`self.OffHandMesh`) true)
  (`SceneComponent.K2_AttachToComponent` (`self.OffHand`) (`self.Mesh`) (`.Off-Hand_13_B721A1014D6248471814A7BBC96B4643` (break `/Game/InventorySystem/Blueprints/Inventory/EquipmentSockets` (`local.LocalEquipmentSockets`))) "SnapToTarget" "SnapToTarget" "SnapToTarget" true))

(fn `OnRep_RightRingMesh`
  (locals (LocalEquipmentSockets :type "/Game/InventorySystem/Blueprints/Inventory/EquipmentSockets Structure" :default (struct :`RightRing` "RightRing" :`LeftRing` "LeftRing" :`Main-Hand` "MainHand" :`Off-Hand` "OffHand")))
  (`SkinnedMeshComponent.SetSkinnedAssetAndUpdate` (`self.RightRing`) (`self.RightRingMesh`) true)
  (`SceneComponent.K2_AttachToComponent` (`self.RightRing`) (`self.Mesh`) (`.RightRing_5_1FCB62154ABF504F5383A3B8EA5B0E39` (break `/Game/InventorySystem/Blueprints/Inventory/EquipmentSockets` (`local.LocalEquipmentSockets`))) "KeepRelative" "KeepRelative" "KeepRelative" true))

(fn `OnRep_ShoulderMesh`
  (`SkinnedMeshComponent.SetSkinnedAssetAndUpdate` (`self.Shoulder`) (`self.ShoulderMesh`) true)
  (`SkinnedMeshComponent.SetLeaderPoseComponent` (`self.Shoulder`) (`self.Mesh`)))

(fn `OnRep_WaistMesh`
  (`SkinnedMeshComponent.SetSkinnedAssetAndUpdate` (`self.Waist`) (`self.WaistMesh`) true)
  (`SkinnedMeshComponent.SetLeaderPoseComponent` (`self.Waist`) (`self.Mesh`)))

(fn `UserConstructionScript`)