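; Golem enemy AI that chases and attacks the player, flashes red when damaged and spawns an apple on death.
; Tick updates player distance and direction for a state machine, with a timer choosing basic or stomp attacks.
; Externally triggered events toggle sphere and capsule hitboxes that damage differently tagged characters.
; Sword overlaps on arm colliders accumulate damage until hand bones hide and severed-arm actors spawn, a prototype part-break system.
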(event `self.ReceiveTick`
  (params (DeltaSeconds :type "Float (single-precision)"))
  ;[1 1 1] Monster Logic
  (`self.SaveDisAndDir`)
  (set `self.IsDeathPlayerChar` false)
  (if (`self.IsDeathPlayerChar`)
    (set `self.CurState` "NewEnumerator3"))
  (switch `/Game/Game/Maps/Level1Contents/Enums/MonsterState` (`self.CurState`)
    (:`NewEnumerator0`
      (if (<= (`self.DistancePlayerChar`) 1000.0)
        (set `self.CurState` "NewEnumerator1")
        (`self.SkillTimeLoop`)))
    (:`NewEnumerator1`
      (if (<= (`self.DistancePlayerChar`) 150.0)
        (`self.StartAttack`)
        (elif (>= (`self.DistancePlayerChar`) 1500.0)
          (set `self.CurState` "NewEnumerator0")
          (else
            (`self.AddMovementInput` (`self.DirToPlayerChar`))))))
    (:`NewEnumerator2`
      (if (`self.IsAttacking`)
        _
        (elif (>= (`self.DistancePlayerChar`) 150.0)
          (set `self.CurState` "NewEnumerator1"))))))

(event `SkillTimeLoop`
  ;[1 1 1] SkillTimeLoop_Event
  (`KismetSystemLibrary.Delay` 1.0)
  (set `self.SkillTime` (+ (`self.SkillTime`) 1.0))
  (`self.SkillTimeLoop`))

(event `self.ReceiveAnyDamage`
  (params (Damage :type "Float (single-precision)") (DamageType :type "DamageType Object Reference") (InstigatedBy :type "Controller Object Reference") (DamageCauser :type "Actor Object Reference"))
  ;[1 1 1] Any Damage_Event
  (bind _output_get (set `self.HP` (- (`self.HP`) Damage)))
  (`self.ChangeDamageColor`)
  (if (<= _output_get 0.0)
    (`self.PlayAnimMontage` "/Game/Game/Mesh/Monster/Monster_Golem_Mesh/AnimMontage/Golem_Stomping_Anim_Montage.Golem_Stomping_Anim_Montage")
    (set `self.CurState` "NewEnumerator4")
    (`PrimitiveComponent.SetCollisionEnabled` (`self.CapsuleComponent`) "NoCollision")
    (`PrimitiveComponent.SetCollisionEnabled` (`self.AttackSphere`) "NoCollision")
    (`PrimitiveComponent.SetCollisionEnabled` (`self.AttackCapsule`) "NoCollision")
    (`KismetSystemLibrary.Delay` 5.0)
    (`self.K2_DestroyActor`)
    (`|SpawnActorFromClass` "/Game/Game/BluePrints/PlayerCharacter/InventorySystem/Blueprints/ItemClasses/Item_Food_Apple.Item_Food_Apple_C" (`self.GetTransform`) "AlwaysSpawn" "OverrideRootScale" null null 0 null)))

(event `StartAttack`
  ;[1 1 1] StartAttack_Event
  (bind _asthird_person_character (cast `/Game/Game/BluePrints/PlayerCharacter/ThirdPersonCharacter` (`GameplayStatics.GetPlayerCharacter` 0)))
  (if (not (`/Game/Game/BluePrints/PlayerCharacter/ThirdPersonCharacter.IsDeath` _asthird_person_character))
    (set `self.IsAttacking` true)
    (if (>= (`self.SkillTime`) 10.0)
      (set `self.CurState` "NewEnumerator5")
      (`self.K2_SetActorRotation` (`KismetMathLibrary.Conv_VectorToRotator` (`self.DirToPlayerChar`)))
      (set `self.SkillTime` 0.0)
      (`KismetSystemLibrary.Delay` 2.0)
      (`self.PlayAnimMontage` "/Game/Game/Mesh/Monster/Monster_Golem_Mesh/AnimMontage/Golem_Stomping_Anim_Montage.Golem_Stomping_Anim_Montage")
      (else
        (set `self.CurState` "NewEnumerator2")
        (`self.K2_SetActorRotation` (`KismetMathLibrary.Conv_VectorToRotator` (`self.DirToPlayerChar`)))
        (`self.PlayAnimMontage` "/Game/Game/Mesh/Monster/Monster_Golem_Mesh/AnimMontage/Golem_Attack_Anim_Montage.Golem_Attack_Anim_Montage")))))

(event `OnAnimEnd_Attack`
  ;[1 1 1] OnAnimEndAttack_Event
  (set `self.IsAttacking` false)
  (if (`self.IsDeathPlayerChar`)
    (set `self.CurState` "NewEnumerator3")
    (elif (>= (`self.DistancePlayerChar`) 180.0)
      (set `self.CurState` "NewEnumerator1")
      (else
        (`self.StartAttack`)))))

(event `self.AttackSphere.OnComponentBeginOverlap`
  (params (OverlappedComponent :type "PrimitiveComponent Object Reference") (OtherActor :type "Actor Object Reference") (OtherComp :type "PrimitiveComponent Object Reference") (OtherBodyIndex :type Integer) (bFromSweep :type Boolean) (SweepResult :type "HitResult Structure (by ref)"))
  ;[1 1 1] ApplyDamage_BasicAttack
  (if (`self.IsAttacking`)
    (if (!= OtherActor self)
      (if (!= (`|GetArrayItem` (`self.Tags`)) (`|GetArrayItem` (`Actor.Tags` OtherActor)))
        (if (== (`|GetArrayItem` (`ActorComponent.ComponentTags` OtherComp)) "Character")
          (`GameplayStatics.ApplyDamage` OtherActor (`self.Atk`) null self))))))

(event `OnColStart_Attack`
  ;[1 1 1] baseCollision_processing
  (`PrimitiveComponent.SetCollisionEnabled` (`self.AttackSphere`) "QueryAndPhysics"))

(event `OnColStart_Skill1Attack`
  ;[1 1 1] Skill1_Collision_processing
  (`PrimitiveComponent.SetCollisionEnabled` (`self.AttackCapsule`) "QueryAndPhysics"))

(event `self.AttackCapsule.OnComponentBeginOverlap`
  (params (OverlappedComponent :type "PrimitiveComponent Object Reference") (OtherActor :type "Actor Object Reference") (OtherComp :type "PrimitiveComponent Object Reference") (OtherBodyIndex :type Integer) (bFromSweep :type Boolean) (SweepResult :type "HitResult Structure (by ref)"))
  ;[1 1 1] ApplyDamage_skillAttack
  (if (`self.IsAttacking`)
    (if (!= OtherActor self)
      (if (!= (`|GetArrayItem` (`self.Tags`)) (`|GetArrayItem` (`Actor.Tags` OtherActor)))
        (if (== (`|GetArrayItem` (`ActorComponent.ComponentTags` OtherComp)) "Character")
          (`GameplayStatics.ApplyDamage` OtherActor (`self.Atk`) null self))))))

(event `SaveDisAndDir`
  (bind _returnvalue (`GameplayStatics.GetPlayerCharacter` 0))
  (bind _returnvalue_2 (`KismetMathLibrary.MakeVector` (.x (- (`self.K2_GetActorLocation` _returnvalue) (`self.K2_GetActorLocation`))) (.y (- (`self.K2_GetActorLocation` _returnvalue) (`self.K2_GetActorLocation`)))))
  ;[1 1 1] SaveDisAndDir_Event
  (bind _asthird_person_character (cast `/Game/Game/BluePrints/PlayerCharacter/ThirdPersonCharacter` _returnvalue))
  (set `self.IsDeathPlayerChar` (`/Game/Game/BluePrints/PlayerCharacter/ThirdPersonCharacter.IsDeath` _asthird_person_character))
  (set `self.DistancePlayerChar` (`KismetMathLibrary.VSize` _returnvalue_2))
  (set `self.DirToPlayerChar` (`KismetMathLibrary.Vector_NormalUnsafe` _returnvalue_2)))

(event `OnColEnd_Attack`
  ;[1 1 1] baseCollision_processing
  (`PrimitiveComponent.SetCollisionEnabled` (`self.AttackSphere`) "NoCollision"))

(event `OnColEnd_Skill1Attack`
  ;[1 1 1] Skill1_Collision_processing
  (`PrimitiveComponent.SetCollisionEnabled` (`self.AttackCapsule`) "NoCollision"))

(event `self.CapsuleComponent.OnComponentBeginOverlap`
  (params (OverlappedComponent :type "PrimitiveComponent Object Reference") (OtherActor :type "Actor Object Reference") (OtherComp :type "PrimitiveComponent Object Reference") (OtherBodyIndex :type Integer) (bFromSweep :type Boolean) (SweepResult :type "HitResult Structure (by ref)"))
  ;[1 1 1] 본 기본적인 알고리즘
)

(event `ChangeDamageColor`
  ;[1 1 1] ChangeDamageColor_Event
  (`PrimitiveComponent.SetMaterial` (`self.Mesh`) 0 "/Game/Game/Mesh/Monster/Monster_Golem_Mesh/Golem_red.Golem_red")
  (`KismetSystemLibrary.Delay` 0.2)
  (`PrimitiveComponent.SetMaterial` (`self.Mesh`) 0 "/Game/Game/Mesh/Monster/Monster_Golem_Mesh/Golem_redblu.Golem_redblu"))

(event `self.RArmCollision.OnComponentEndOverlap`
  (params (OverlappedComponent :type "PrimitiveComponent Object Reference") (OtherActor :type "Actor Object Reference") (OtherComp :type "PrimitiveComponent Object Reference") (OtherBodyIndex :type Integer))
  (bind _mesh (`self.Mesh`))
  (bind _bip001_r_hand (`self.Bip001-R-Hand`))
  (bind _rarmaccumulatedmg (`self.RArmAccumulateDmg`))
  (bind _returnvalue (+ (`self.RArmAccumulateDmg`) 10.0))
  ;[1 1 1] 팔 부위파괴 Temp
  (bind _asweapon_sword_1 (cast `/Game/Game/BluePrints/PlayerCharacter/Weapon_Sword1` OtherActor))
  (if (and (< (`self.RArmAccumulateDmg`) 300.0) (`/Game/Game/BluePrints/PlayerCharacter/Weapon_Sword1.CanCut` _asweapon_sword_1))
    (set `self.RArmAccumulateDmg` _returnvalue)
    (`KismetSystemLibrary.PrintString` (`KismetStringLibrary.Conv_DoubleToString` _returnvalue)))
  (if (and (>= _rarmaccumulatedmg 100.0) (< _rarmaccumulatedmg 200.0))
    (if (`/Game/Game/BluePrints/PlayerCharacter/Weapon_Sword1.CanCut` _asweapon_sword_1)
      (`KismetSystemLibrary.PrintString` "RightArm")
      (`SkinnedMeshComponent.HideBoneByName` _mesh _bip001_r_hand "PBO_None")
      (`/Engine/EditorBlueprintResources/StandardMacros.DoOnce` false
        (:`Completed`
          (`GameplayStatics.SpawnEmitterAtLocation` null (`SceneComponent.GetSocketLocation` _mesh _bip001_r_hand))
          (`|SpawnActorFromClass` "/Game/Game/Mesh/Monster/Monster_Golem_Mesh/Golem_Parts/Golem_Left_Arm_DM_BP.Golem_Left_Arm_DM_BP_C" (`SceneComponent.GetSocketTransform` _mesh _bip001_r_hand "RTS_World") "Undefined" "OverrideRootScale" null null))))))

(event `self.LArmCollision.OnComponentEndOverlap`
  (params (OverlappedComponent :type "PrimitiveComponent Object Reference") (OtherActor :type "Actor Object Reference") (OtherComp :type "PrimitiveComponent Object Reference") (OtherBodyIndex :type Integer))
  (bind _bip001_l_hand (`self.Bip001-L-Hand`))
  (bind _mesh (`self.Mesh`))
  (bind _returnvalue (+ (`self.LArmAccumulateDmg`) 10.0))
  ;[1 1 1] 팔 부위파괴 Temp
  (bind _asweapon_sword_1 (cast `/Game/Game/BluePrints/PlayerCharacter/Weapon_Sword1` OtherActor))
  (if (`/Game/Game/BluePrints/PlayerCharacter/Weapon_Sword1.CanCut` _asweapon_sword_1)
    (if (< (`self.LArmAccumulateDmg`) 100.0)
      (set `self.LArmAccumulateDmg` _returnvalue)
      (`KismetSystemLibrary.PrintString` (`KismetStringLibrary.Conv_DoubleToString` _returnvalue)))
    (if (>= (`self.LArmAccumulateDmg`) 100.0)
      (`KismetSystemLibrary.PrintString` "leftArm")
      (`SkinnedMeshComponent.HideBoneByName` _mesh _bip001_l_hand "PBO_None")
      (`/Engine/EditorBlueprintResources/StandardMacros.DoOnce` false
        (:`Completed`
          (`|SpawnActorFromClass` "/Game/Game/Mesh/Monster/Monster_Golem_Mesh/Golem_Parts/Golem_Left_Arm_DM_BP.Golem_Left_Arm_DM_BP_C" (`SceneComponent.GetSocketTransform` _mesh _bip001_l_hand "RTS_World") "Undefined" "OverrideRootScale" null null))))))

(fn `UserConstructionScript`)