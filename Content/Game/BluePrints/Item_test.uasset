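; Test pickup item that a ThirdPersonCharacter loots into an eight-slot inventory.
; Tick polls overlap using the begin-overlap actor and, while that character is looting, spawns a loot particle at the character.
; It then writes item ID 2 into the first empty InventoryItem variable on ThirdPersonGameMode and destroys itself.
; With all slots full the item stays, though the particle still spawns.
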(event `self.ReceiveActorBeginOverlap`
  (params (OtherActor :type "Actor Object Reference")))

(event `self.ReceiveTick`
  (params (DeltaSeconds :type "Float (single-precision)"))
  (bind _asthird_person_character (cast `/Game/Game/BluePrints/ThirdPersonCharacter` (stale `self.ReceiveActorBeginOverlap` OtherActor)))
  (if (or (`self.IsOverlappingActor` (stale `self.ReceiveActorBeginOverlap` OtherActor)) (`self.IsOverlappingActor` self null))
    (if (`/Game/Game/BluePrints/ThirdPersonCharacter.IsLooting` _asthird_person_character)
      (`GameplayStatics.SpawnEmitterAtLocation` "/Game/InfinityBladeEffects/Effects/FX_Treasure/Loot/P_Loot_Pickup.P_Loot_Pickup" (`self.K2_GetActorLocation` _asthird_person_character))
      (bind _asthird_person_game_mode (cast `/Game/Game/BluePrints/ThirdPersonGameMode` (`GameplayStatics.GetGameMode`)))
      (if (== (`/Game/Game/BluePrints/ThirdPersonGameMode.InventoryItem1` _asthird_person_game_mode) 0)
        (set `/Game/Game/BluePrints/ThirdPersonGameMode.InventoryItem1` 2 _asthird_person_game_mode)
        (`self.K2_DestroyActor` :!label _label)
        (elif (== (`/Game/Game/BluePrints/ThirdPersonGameMode.InventoryItem2` _asthird_person_game_mode) 0)
          (set `/Game/Game/BluePrints/ThirdPersonGameMode.InventoryItem2` 2 _asthird_person_game_mode)
          (goto _label)
          (elif (== (`/Game/Game/BluePrints/ThirdPersonGameMode.InventoryItem3` _asthird_person_game_mode) 0)
            (set `/Game/Game/BluePrints/ThirdPersonGameMode.InventoryItem3` 2 _asthird_person_game_mode)
            (goto _label)
            (elif (== (`/Game/Game/BluePrints/ThirdPersonGameMode.InventoryItem4` _asthird_person_game_mode) 0)
              (set `/Game/Game/BluePrints/ThirdPersonGameMode.InventoryItem4` 2 _asthird_person_game_mode)
              (goto _label)
              (elif (== (`/Game/Game/BluePrints/ThirdPersonGameMode.InventoryItem5` _asthird_person_game_mode) 0)
                (set `/Game/Game/BluePrints/ThirdPersonGameMode.InventoryItem5` 2 _asthird_person_game_mode)
                (goto _label)
                (elif (== (`/Game/Game/BluePrints/ThirdPersonGameMode.InventoryItem6` _asthird_person_game_mode) 0)
                  (set `/Game/Game/BluePrints/ThirdPersonGameMode.InventoryItem6` 2 _asthird_person_game_mode)
                  (goto _label)
                  (elif (== (`/Game/Game/BluePrints/ThirdPersonGameMode.InventoryItem7` _asthird_person_game_mode) 0)
                    (set `/Game/Game/BluePrints/ThirdPersonGameMode.InventoryItem7` 2 _asthird_person_game_mode)
                    (goto _label)
                    (elif (== (`/Game/Game/BluePrints/ThirdPersonGameMode.InventoryItem8` _asthird_person_game_mode) 0)
                      (set `/Game/Game/BluePrints/ThirdPersonGameMode.InventoryItem8` 2 _asthird_person_game_mode)
                      (goto _label))))))))))))

(event `self.Box.OnComponentBeginOverlap`
  (params (OverlappedComponent :type "PrimitiveComponent Object Reference") (OtherActor :type "Actor Object Reference") (OtherComp :type "PrimitiveComponent Object Reference") (OtherBodyIndex :type Integer) (bFromSweep :type Boolean) (SweepResult :type "HitResult Structure (by ref)")))

(fn `UserConstructionScript`)