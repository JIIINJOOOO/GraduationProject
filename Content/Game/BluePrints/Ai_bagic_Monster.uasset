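; AI controller for a basic monster that senses enemies of other teams and moves its pawn toward them.
; Sight locks on, draws the sword, approaches and enables attacking after five seconds; hearing only triggers movement until an enemy has been seen.
; A DoOnce-gated GotoLocation retries failed moves on a delay, using random reachable points near the target or partway toward distant ones.
; Pawn commands and team checks go through message calls.
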(event `self.ReceiveBeginPlay`
  (set `self.ch` (`self.K2_GetPawn`)))

(event `self.GoToLocation`
  (params (Targetlocation :type "Vector Structure"))
  (bind _randomlocation (`self.Get TargetLocation` Targetlocation))
  (bind _output_get (set `self.destination` Targetlocation))
  (`/Engine/EditorBlueprintResources/StandardMacros.DoOnce` false :!label _label
    (:`Completed`
      (`|AIMoveTo` null _output_get null
        (:`OnSuccess`
          (goto _label :!via `Reset`))
        (:`OnFail`
          (`|AIMoveTo` null _randomlocation null 200.0 :!label _label_2
            (:`OnSuccess`
              (if (< (`self.Get Distance And Direction` _randomlocation (`self.K2_GetActorLocation` (`self.ch`))) 200.0)
                (goto _label :!via `Reset`)
                (else
                  _)))
            (:`OnFail`
              _))
          (`KismetSystemLibrary.Delay` 2.0)
          (goto _label_2))))))

(fn `Get Distance And Direction`
  (params (`Target Location` :type "Vector Structure") (`currect Location` :type "Vector Structure"))
  (returns (distance :type "Float (double-precision)") (direction :type "Vector Structure"))
  (bind _returnvalue (- `Target Location` `currect Location`))
  (return (`KismetMathLibrary.VSize` _returnvalue) (`KismetMathLibrary.Normal` _returnvalue)))

(fn `Get TargetLocation`
  (params (terget :type "Vector Structure (by ref)"))
  (returns (RandomLocation :type "Vector Structure"))
  (bind _randomlocation (`NavigationSystemV1.K2_GetRandomReachablePointInRadius` terget 100.0 null null))
  (bind _returnvalue (`self.K2_GetActorLocation` (`self.ch`)))
  (bind (_distance _direction) (`self.Get Distance And Direction` _randomlocation _returnvalue))
  (if (< _distance 2500.0)
    (return _randomlocation)
    (else
      (return (`NavigationSystemV1.K2_GetRandomReachablePointInRadius` (+ _returnvalue (* _direction 1500.0)) 100.0 null null)))))

(fn `OnReaction_AI`
  (returns (Reaction :type Boolean))
  (return false))

(fn `UserConstructionScript`)