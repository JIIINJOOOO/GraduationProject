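; Player skill projectile that damages monsters and explodes in flame on contact.
; On overlap, it casts the other actor to Monster_BP_2 or Golem_BP, applies SkillDmg, spawns the explosion emitter at its Sphere and destroys itself.
; Each tick it destroys itself without an explosion once its horizontal distance from the player pawn, cached at BeginPlay, exceeds Range.
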(event `self.ReceiveBeginPlay`
  (bind _asbp_player (cast `/Game/Game/BluePrints/player/BP_player` (`GameplayStatics.GetPlayerPawn` 0))))

(event `self.ReceiveActorBeginOverlap`
  (params (OtherActor :type "Actor Object Reference"))
  (`|ExecutionSequence`
    (:`then_0`
      (bind _asmonster_bp_2 (cast `/Game/Game/BluePrints/Goblin/Monster_BP_2` OtherActor))
      (`GameplayStatics.ApplyDamage` _asmonster_bp_2 (`self.SkillDmg`) null self))
    (:`then_1`
      (bind _asgolem_bp (cast `/Game/Game/BluePrints/Boss_Golem/Golem_BP` OtherActor))
      (`GameplayStatics.ApplyDamage` _asgolem_bp (`self.SkillDmg`) null self)))
  (`GameplayStatics.SpawnEmitterAtLocation` "/Game/Game/particle/Character_Skill/P_FlameExplode.P_FlameExplode" (`SceneComponent.K2_GetComponentLocation` (`self.Sphere`)) (struct :`Roll` 90.0))
  (`self.K2_DestroyActor`))

(event `self.ReceiveTick`
  (params (DeltaSeconds :type "Float (single-precision)"))
  (if (> (`self.GetHorizontalDistanceTo` (stale `self.ReceiveBeginPlay` _asbp_player)) (`self.Range`))
    (`self.K2_DestroyActor`)))

(fn `UserConstructionScript`)