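; Sword weapon Blueprint that damages goblin and mutant monsters it touches while the player is attacking.
; When its Box collision begins overlapping an actor, a sequence checks for each monster class separately.
; On a match, it reads IsAttacking from the player's ThirdPersonCharacter and, if true, applies AttackDmg with the sword as damage causer.
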(event `self.Box.OnComponentBeginOverlap`
  (params (OverlappedComponent :type "PrimitiveComponent Object Reference") (OtherActor :type "Actor Object Reference") (OtherComp :type "PrimitiveComponent Object Reference") (OtherBodyIndex :type Integer) (bFromSweep :type Boolean) (SweepResult :type "HitResult Structure (by ref)"))
  (`|ExecutionSequence`
    (:`then_0`
      (bind _asgoblin_monster_bp (cast `/Game/Game/BluePrints/Goblin_Monster_BP` OtherActor))
      (bind _asthird_person_character (cast `/Game/Game/BluePrints/ThirdPersonCharacter` (`GameplayStatics.GetPlayerCharacter` 0)))
      (if (`/Game/Game/BluePrints/ThirdPersonCharacter.IsAttacking` _asthird_person_character)
        (`GameplayStatics.ApplyDamage` _asgoblin_monster_bp (`self.AttackDmg`) null self)))
    (:`then_1`
      (bind _asmutant_monster_bp (cast `/Game/Game/BluePrints/mutant_Monster_BP` OtherActor))
      (bind _asthird_person_character_2 (cast `/Game/Game/BluePrints/ThirdPersonCharacter` (`GameplayStatics.GetPlayerCharacter` 0)))
      (if (`/Game/Game/BluePrints/ThirdPersonCharacter.IsAttacking` _asthird_person_character_2)
        (`GameplayStatics.ApplyDamage` _asmutant_monster_bp (`self.AttackDmg`) null self)))))

(fn `UserConstructionScript`)