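; Mutant monster AI that fights the player with punches and a timed skill attack, and drops an item on death.
; Event-driven montages chain attacks, with collision events toggling sphere and capsule hitboxes that damage differently tagged characters.
; Taking damage flashes the material; at zero HP it dies and is later destroyed.
; The distance-based idle, chase and attack state machine is disconnected from the empty Tick, so it never runs.
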(event `self.ReceiveTick`
  (params (DeltaSeconds :type "Float (single-precision)"))
  ;[1 1 1] Monster Logic
)

(event `SkillTimeLoop`
  ;[1 1 1] SkillTimeLoop_Event
  (`KismetSystemLibrary.Delay` 1.0)
  (set `self.SkillTime` (+ (`self.SkillTime`) 1.0))
  (`self.SkillTimeLoop`))

(event `self.ReceiveAnyDamage`
  (params (Damage :type "Float (single-precision)") (DamageType :type "DamageType Object Reference") (InstigatedBy :type "Controller Object Reference") (DamageCauser :type "Actor Object Reference"))
  ;[1 1 1] Any Damage_Event
  (bind _output_get (set `self.HP` (- (`self.HP`) Damage)))
  (`self.ChangeDamageColor`)
  (if (<= _output_get 0.0)
    (`self.PlayAnimMontage` "/Game/Game/Mesh/Monster/Monster_Mutant_Mesh/AnimMontage/Mutant_dying_Montage.Mutant_dying_Montage")
    (set `self.CurState` "NewEnumerator4")
    (`PrimitiveComponent.SetCollisionEnabled` (`self.CapsuleComponent`) "NoCollision")
    (`PrimitiveComponent.SetCollisionEnabled` (`self.Sphere`) "NoCollision")
    (`PrimitiveComponent.SetCollisionEnabled` (`self.Capsule`) "NoCollision")
    (`KismetSystemLibrary.Delay` 5.0)
    (`self.K2_DestroyActor`)
    (`|SpawnActorFromClass` "/Game/Game/BluePrints/Item_test.Item_test_C" (`self.GetTransform`) "AlwaysSpawn" "OverrideRootScale" null null)))

(event `StartAttack`
  ;[1 1 1] StartAttack_Event
  (bind _asthird_person_character (cast `/Game/Game/BluePrints/PlayerCharacter/ThirdPersonCharacter` (`GameplayStatics.GetPlayerCharacter` 0)))
  (if (not (`/Game/Game/BluePrints/PlayerCharacter/ThirdPersonCharacter.IsDeath` _asthird_person_character))
    (set `self.IsAttacking` true)
    (if (>= (`self.SkillTime`) 10.0)
      (set `self.CurState` "NewEnumerator5")
      (`self.K2_SetActorRotation` (`KismetMathLibrary.Conv_VectorToRotator` (`self.DirToPlayerChar`)))
      (`PrimitiveComponent.SetMaterial` (`self.Mesh`) 0 "/Game/Game/Mesh/Monster/Monster_Mutant_Mesh/mutant_M_Skill_inst.mutant_M_Skill_inst")
      (set `self.SkillTime` 0.0)
      (`self.PlayAnimMontage` "/Game/Game/Mesh/Monster/Monster_Mutant_Mesh/AnimMontage/Mutant_FlexingMuscles_Montage.Mutant_FlexingMuscles_Montage" 1.0 "Start")
      (`KismetSystemLibrary.Delay` 2.0)
      (`PrimitiveComponent.SetMaterial` (`self.Mesh`) 0 "/Game/Game/Mesh/Monster/Monster_Mutant_Mesh/mutant_M.mutant_M")
      (`self.PlayAnimMontage` "/Game/Game/Mesh/Monster/Monster_Mutant_Mesh/AnimMontage/Mutant_Swiping_Montage.Mutant_Swiping_Montage")
      (else
        (set `self.CurState` "NewEnumerator2")
        (`self.K2_SetActorRotation` (`KismetMathLibrary.Conv_VectorToRotator` (`self.DirToPlayerChar`)))
        (`self.PlayAnimMontage` "/Game/Game/Mesh/Monster/Monster_Mutant_Mesh/AnimMontage/Mutant_Punch_Montage.Mutant_Punch_Montage")))))

(event `OnAnimEnd_Attack`
  ;[1 1 1] OnAnimEndAttack_Event
  (`PrimitiveComponent.SetMaterial` (`self.Mesh`) 0 "/Game/Game/Mesh/Monster/Monster_Mutant_Mesh/mutant_M.mutant_M")
  (set `self.IsAttacking` false)
  (if (`self.IsDeathPlayerChar`)
    (set `self.CurState` "NewEnumerator3")
    (elif (>= (`self.DistancePlayerChar`) 180.0)
      (set `self.CurState` "NewEnumerator1")
      (else
        (`self.StartAttack`)))))

(event `self.Sphere.OnComponentBeginOverlap`
  (params (OverlappedComponent :type "PrimitiveComponent Object Reference") (OtherActor :type "Actor Object Reference") (OtherComp :type "PrimitiveComponent Object Reference") (OtherBodyIndex :type Integer) (bFromSweep :type Boolean) (SweepResult :type "HitResult Structure (by ref)"))
  ;[1 1 1] ApplyDamage_BasicAttack
  (if (`self.IsAttacking`)
    (if (!= OtherActor self)
      (if (!= (`|GetArrayItem` (`self.Tags`)) (`|GetArrayItem` (`Actor.Tags` OtherActor)))
        (if (== (`|GetArrayItem` (`ActorComponent.ComponentTags` OtherComp)) "Character")
          (`GameplayStatics.ApplyDamage` OtherActor (`self.Atk`) null self))))))

(event `OnColStart_Attack`
  ;[1 1 1] baseCollision_processing
  (`PrimitiveComponent.SetCollisionEnabled` (`self.Sphere`) "QueryAndPhysics"))

(event `OnColStart_Skill1Attack`
  ;[1 1 1] Skill1_Collision_processing
  (`PrimitiveComponent.SetCollisionEnabled` (`self.Capsule`) "QueryAndPhysics"))

(event `self.Capsule.OnComponentBeginOverlap`
  (params (OverlappedComponent :type "PrimitiveComponent Object Reference") (OtherActor :type "Actor Object Reference") (OtherComp :type "PrimitiveComponent Object Reference") (OtherBodyIndex :type Integer) (bFromSweep :type Boolean) (SweepResult :type "HitResult Structure (by ref)"))
  ;[1 1 1] ApplyDamage_skillAttack
  (if (`self.IsAttacking`)
    (if (!= OtherActor self)
      (if (!= (`|GetArrayItem` (`self.Tags`)) (`|GetArrayItem` (`Actor.Tags` OtherActor)))
        (if (== (`|GetArrayItem` (`ActorComponent.ComponentTags` OtherComp)) "Character")
          (`GameplayStatics.ApplyDamage` OtherActor (`self.Atk`) null self))))))

(event `SaveDisAndDir`
  (bind _returnvalue (`GameplayStatics.GetPlayerCharacter` 0))
  (bind _returnvalue_2 (`KismetMathLibrary.MakeVector` (.x (- (`self.K2_GetActorLocation` _returnvalue) (`self.K2_GetActorLocation`))) (.y (- (`self.K2_GetActorLocation` _returnvalue) (`self.K2_GetActorLocation`)))))
  ;[1 1 1] SaveDisAndDir_Event
  (bind _asthird_person_character (cast `/Game/Game/BluePrints/PlayerCharacter/ThirdPersonCharacter` _returnvalue))
  (set `self.IsDeathPlayerChar` (`/Game/Game/BluePrints/PlayerCharacter/ThirdPersonCharacter.IsDeath` _asthird_person_character))
  (set `self.DistancePlayerChar` (`KismetMathLibrary.VSize` _returnvalue_2))
  (set `self.DirToPlayerChar` (`KismetMathLibrary.Vector_NormalUnsafe` _returnvalue_2)))

(event `OnColEnd_Attack`
  ;[1 1 1] baseCollision_processing
  (`PrimitiveComponent.SetCollisionEnabled` (`self.Sphere`) "NoCollision"))

(event `OnColEnd_Skill1Attack`
  ;[1 1 1] Skill1_Collision_processing
  (`PrimitiveComponent.SetCollisionEnabled` (`self.Capsule`) "NoCollision"))

(event `ChangeDamageColor`
  ;[1 1 1] ChangeDamageColor_Event
  (`PrimitiveComponent.SetMaterial` (`self.Mesh`) 0 "/Game/Game/Mesh/Monster/Monster_Mutant_Mesh/mutant_M_Inst.mutant_M_Inst")
  (`KismetSystemLibrary.Delay` 0.2)
  (`PrimitiveComponent.SetMaterial` (`self.Mesh`) 0 "/Game/Game/Mesh/Monster/Monster_Mutant_Mesh/mutant_M.mutant_M"))

(fn `UserConstructionScript`)