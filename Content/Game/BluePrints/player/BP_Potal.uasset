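; Portal actor that opens when its activation collider is overlapped and teleports actors entering its teleport collider.
; The plane starts nearly invisible in scale, then a one-time activation plays sound and ice vortex particles while a timeline scales it up.
; Each tick, CameraTracker copies the player camera, and its relative transform drives PotalCapture for a see-through perspective.
; Teleporting sends PotalCapture's world transform to the overlapping actor through TeleportMessage.
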(event `self.ReceiveBeginPlay`
  (bind _plane1 (`self.Plane1`))
  (`SceneComponent.SetRelativeScale3D` _plane1 (* (`SceneComponent.RelativeScale3D` _plane1) 0.01)))

(event `self.ReceiveTick`
  (params (DeltaSeconds :type "Float (single-precision)"))
  (`self.Set Transform` (`SceneComponent.K2_GetComponentToWorld` (`PlayerCameraManager.TransformComponent` (`GameplayStatics.GetPlayerCameraManager` 0)))))

(event `self.collider_teleport.OnComponentBeginOverlap`
  (params (OverlappedComponent :type "PrimitiveComponent Object Reference") (OtherActor :type "Actor Object Reference") (OtherComp :type "PrimitiveComponent Object Reference") (OtherBodyIndex :type Integer) (bFromSweep :type Boolean) (SweepResult :type "HitResult Structure (by ref)"))
  (message `/Game/Game/Interface/BPI_Teleport.Teleport` OtherActor (`SceneComponent.K2_GetComponentToWorld` (`self.Potal_capture`))))

(event `activate_portal`
  (`/Engine/EditorBlueprintResources/StandardMacros.DoOnce` false
    (:`Completed`
      (`GameplayStatics.PlaySoundAtLocation` "/Game/Game/Sound/potal/Item_Teleport.Item_Teleport" (`SceneComponent.K2_GetComponentLocation` (`self.Plane1`)) (struct) 1.0 1.0 0.0 null null null)
      (`ActorComponent.Activate` (`self.P_AuraCircle_Ice_Vortex_01`) true)
      (bind (_direction _scale_multpler) (`Timeline|timeline_portal` :!via `PlayFromStart`)
        (:`Update`
          (`SceneComponent.SetRelativeScale3D` (`self.Plane1`) (* (2.5 2.5 1.0) _scale_multpler)))))))

(event `self.collider_activate.OnComponentBeginOverlap`
  (params (OverlappedComponent :type "PrimitiveComponent Object Reference") (OtherActor :type "Actor Object Reference") (OtherComp :type "PrimitiveComponent Object Reference") (OtherBodyIndex :type Integer) (bFromSweep :type Boolean) (SweepResult :type "HitResult Structure (by ref)"))
  (`self.activate_portal`))

(fn `UserConstructionScript`
  (bind _camera (`self.camera`))
  (`/Engine/EditorBlueprintResources/StandardMacros.IsValid` _camera
    (:`Is Valid`
      (`self.Set Transform` (`SceneComponent.K2_GetComponentToWorld` (`CameraActor.SceneComponent` _camera))))))