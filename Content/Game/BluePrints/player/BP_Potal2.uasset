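; BP_Potal2 is a portal actor with a scene capture component and a teleport collider.
; Overlapping the collider sends the other actor a TeleportMessage carrying PotalCapture's world transform.
; Tick passes the player camera's transform to SetTransform, as does the construction script with an optional Camera reference.
; SetTransform's entry is unwired, so its nodes for repositioning the capture relative to that transform never run.
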(event `self.ReceiveBeginPlay`)

(event `self.ReceiveTick`
  (params (DeltaSeconds :type "Float (single-precision)"))
  (`self.Set Transform` (`SceneComponent.K2_GetComponentToWorld` (`PlayerCameraManager.TransformComponent` (`GameplayStatics.GetPlayerCameraManager` 0)))))

(event `self.collider_teleport.OnComponentBeginOverlap`
  (params (OverlappedComponent :type "PrimitiveComponent Object Reference") (OtherActor :type "Actor Object Reference") (OtherComp :type "PrimitiveComponent Object Reference") (OtherBodyIndex :type Integer) (bFromSweep :type Boolean) (SweepResult :type "HitResult Structure (by ref)"))
  (message `/Game/Game/Interface/BPI_Teleport.Teleport` OtherActor (`SceneComponent.K2_GetComponentToWorld` (`self.Potal_capture`))))

(fn `UserConstructionScript`
  (bind _camera (`self.camera`))
  (`/Engine/EditorBlueprintResources/StandardMacros.IsValid` _camera
    (:`Is Valid`
      (`self.Set Transform` (`SceneComponent.K2_GetComponentToWorld` (`CameraActor.SceneComponent` _camera))))))