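; Great hammer weapon actor for the player, supplying attack montages, socket transforms and visual feedback.
; Regular and combo montages cycle by attack count modulo array length, with a separate fixed charge montage.
; A dynamic material created at BeginPlay drives the charge effect, and the trail toggle plays a one-shot skeletal animation when enabled.
; On overlap, CanCut mirrors whether the player is attacking, regardless of which actor overlaps.
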(event `self.ReceiveBeginPlay`
  (bind _returnvalue (`PrimitiveComponent.CreateDynamicMaterialInstance` (`self.SM_Sword`) 0 "/Game/Weapon_Pack/Materials/Weapons/M_WeaponSet_1.M_WeaponSet_1" "None"))
  (set `self.weapon matenial` _returnvalue))

(event `self.ReceiveActorBeginOverlap`
  (params (OtherActor :type "Actor Object Reference"))
  (bind _asbp_player (cast `/Game/Game/BluePrints/player/BP_player` (`GameplayStatics.GetPlayerCharacter` 0)))
  (if (`/Game/Game/BluePrints/player/BP_player.IsAttacking` _asbp_player)
    (set `self.CanCut` true)
    (else
      (set `self.CanCut` false))))

(event `/Game/Game/Interface/BPI_weapon.ToggleChargeWeapon`
  (params (enable :type Boolean))
  (`MaterialInstanceDynamic.SetScalarParameterValue` (`self.weapon matenial`) "Charge multiplier" (select `bool` enable :`true` 50.0 :!type "Float (single-precision)")))

(event `/Game/Game/Interface/BPI_weapon.ToggleWeaponTrail_base`
  (params (enable :type Boolean))
  (if enable
    (`SkeletalMeshComponent.PlayAnimation` (`self.SK_Trail`) "/Game/Game/particle/cube/Cube_Anim.Cube_Anim" false)))

(fn `GetAttackMontage`
  (params (`attack Count` :type Integer) (isComboAttack :type Boolean))
  (returns (`Attack Montage` :type "AnimMontage Object Reference"))
  (bind _regular_attacks (`self.regular attacks`))
  (bind _combo_attacks (`self.combo attacks`))
  (if isComboAttack
    (return (`|GetArrayItem` _combo_attacks (mod `attack Count` (`KismetArrayLibrary.Array_Length` _combo_attacks))))
    (else
      (return (`|GetArrayItem` _regular_attacks (mod `attack Count` (`KismetArrayLibrary.Array_Length` _regular_attacks)))))))

(fn `GetChargeMontage`
  (returns (`charge Montage` :type "AnimMontage Object Reference"))
  (return "/Game/Game/Mesh/player_anim/Mixamo/Sword_And_Shield_Slash_Montage_Charge.Sword_And_Shield_Slash_Montage_Charge"))

(fn `GetWeaponSocketTransform`
  (params (`Socket name` :type Name))
  (returns (transform :type "Transform Structure"))
  (return (`SceneComponent.GetSocketTransform` (`self.SM_Sword`) `Socket name` "RTS_World")))

(fn `UserConstructionScript`)