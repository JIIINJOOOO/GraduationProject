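; Player sword weapon that damages monsters and slices procedural meshes while the character is attacking.
; Box overlaps apply AttackDmg to Monster_BP and mutant_Monster_BP actors, gated by the ThirdPersonCharacter's IsAttacking flag.
; SliceMeshCollision overlaps cut procedural meshes along the sword mesh's up-vector plane, creating a capped, physics-simulated half and applying a radial impulse to the original.
; A do-once gate limits slicing until an overlap outside an attack resets it.
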(event `self.Box.OnComponentBeginOverlap`
  (params (OverlappedComponent :type "PrimitiveComponent Object Reference") (OtherActor :type "Actor Object Reference") (OtherComp :type "PrimitiveComponent Object Reference") (OtherBodyIndex :type Integer) (bFromSweep :type Boolean) (SweepResult :type "HitResult Structure (by ref)"))
  (`|ExecutionSequence`
    (:`then_0`
      (bind _asmonster_bp (cast `/Game/Game/BluePrints/Monster_BP` OtherActor))
      (bind _asthird_person_character (cast `/Game/Game/BluePrints/PlayerCharacter/ThirdPersonCharacter` (`GameplayStatics.GetPlayerCharacter` 0)))
      (if (`/Game/Game/BluePrints/PlayerCharacter/ThirdPersonCharacter.IsAttacking` _asthird_person_character)
        (`GameplayStatics.ApplyDamage` _asmonster_bp (`self.AttackDmg`) null self)))
    (:`then_1`
      (bind _asmutant_monster_bp (cast `/Game/Game/BluePrints/mutant_Monster_BP` OtherActor))
      (bind _asthird_person_character_2 (cast `/Game/Game/BluePrints/PlayerCharacter/ThirdPersonCharacter` (`GameplayStatics.GetPlayerCharacter` 0)))
      (if (`/Game/Game/BluePrints/PlayerCharacter/ThirdPersonCharacter.IsAttacking` _asthird_person_character_2)
        (`GameplayStatics.ApplyDamage` _asmutant_monster_bp (`self.AttackDmg`) null self)))))

(event `self.SliceMeshCollision.OnComponentBeginOverlap`
  (params (OverlappedComponent :type "PrimitiveComponent Object Reference") (OtherActor :type "Actor Object Reference") (OtherComp :type "PrimitiveComponent Object Reference") (OtherBodyIndex :type Integer) (bFromSweep :type Boolean) (SweepResult :type "HitResult Structure (by ref)"))
  (bind _skeletalmesh (`self.SkeletalMesh`))
  (bind _returnvalue (`SceneComponent.K2_GetComponentLocation` _skeletalmesh))
  (bind _asthird_person_character (cast `/Game/Game/BluePrints/PlayerCharacter/ThirdPersonCharacter` (`GameplayStatics.GetPlayerCharacter` 0)))
  (if (`/Game/Game/BluePrints/PlayerCharacter/ThirdPersonCharacter.IsAttacking` _asthird_person_character)
    (set `self.CanCut` true)
    (add `PrimitiveComponent.OnComponentBeginOverlap` _skeletalmesh (delegate `OnComponentBeginOverlap_Event_0`))
    (`/Engine/EditorBlueprintResources/StandardMacros.DoOnce` false :!label _label
      (:`Completed`
        (bind _asprocedural_mesh_component (cast `ProceduralMeshComponent` (stale `OnComponentBeginOverlap_Event_0` OtherComp)))
        (bind _outotherhalfprocmesh (`KismetProceduralMeshLibrary.SliceProceduralMesh` _asprocedural_mesh_component _returnvalue (`SceneComponent.GetUpVector` _skeletalmesh) true "CreateNewSectionForCap" "/Game/StarterContent/Materials/M_Concrete_Tiles.M_Concrete_Tiles"))
        (`PrimitiveComponent.SetSimulatePhysics` _outotherhalfprocmesh true)
        (`PrimitiveComponent.AddRadialImpulse` _asprocedural_mesh_component _returnvalue 700.0 50000.0 "RIF_Constant" false)))
    (else
      (set `self.CanCut` false)
      (goto _label :!via `Reset`))))

(event `OnComponentBeginOverlap_Event_0`
  (params (OverlappedComponent :type "PrimitiveComponent Object Reference") (OtherActor :type "Actor Object Reference") (OtherComp :type "PrimitiveComponent Object Reference") (OtherBodyIndex :type Integer) (bFromSweep :type Boolean) (SweepResult :type "HitResult Structure (by ref)")))

(fn `UserConstructionScript`)