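; Sword weapon actor that damages monsters and slices procedural meshes while the player character is attacking.
; Its collision box applies damage to actors tagged Monster, then briefly disables its collision as a hit cooldown.
; A separate Plane component cuts overlapped procedural meshes along its position and up vector, capping the cut, simulating physics on the new half and adding a radial impulse.
; A DoOnce gates slicing until an overlap occurs outside an attack.
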(event `self.ReceiveTick`
  (params (DeltaSeconds :type "Float (single-precision)")))

(event `self.CollisionBox.OnComponentBeginOverlap`
  (params (OverlappedComponent :type "PrimitiveComponent Object Reference") (OtherActor :type "Actor Object Reference") (OtherComp :type "PrimitiveComponent Object Reference") (OtherBodyIndex :type Integer) (bFromSweep :type Boolean) (SweepResult :type "HitResult Structure (by ref)"))
  (bind _asthird_person_character (cast `/Game/Game/BluePrints/PlayerCharacter/ThirdPersonCharacter` (`GameplayStatics.GetPlayerCharacter` 0)))
  (if (and (`/Game/Game/BluePrints/PlayerCharacter/ThirdPersonCharacter.IsAttacking` _asthird_person_character) (== (`|GetArrayItem` (`Actor.Tags` OtherActor)) "Monster"))
    (`GameplayStatics.ApplyDamage` OtherActor (`self.AttackDmg`) null self)
    (`PrimitiveComponent.SetCollisionEnabled` (`self.CollisionBox`) "NoCollision")
    (set `self.CanCollide` false)
    (`KismetSystemLibrary.Delay` 2.0)
    (`PrimitiveComponent.SetCollisionEnabled` (`self.CollisionBox`) "QueryAndPhysics")
    (set `self.CanCollide` true)))

(event `self.Plane.OnComponentBeginOverlap`
  (params (OverlappedComponent :type "PrimitiveComponent Object Reference") (OtherActor :type "Actor Object Reference") (OtherComp :type "PrimitiveComponent Object Reference") (OtherBodyIndex :type Integer) (bFromSweep :type Boolean) (SweepResult :type "HitResult Structure (by ref)"))
  (bind _plane (`self.Plane`))
  (bind _returnvalue (`SceneComponent.K2_GetComponentLocation` _plane))
  (bind _asthird_person_character (cast `/Game/Game/BluePrints/PlayerCharacter/ThirdPersonCharacter` (`GameplayStatics.GetPlayerCharacter` 0)))
  (if (`/Game/Game/BluePrints/PlayerCharacter/ThirdPersonCharacter.IsAttacking` _asthird_person_character)
    (set `self.CanCut` true)
    (add `PrimitiveComponent.OnComponentBeginOverlap` _plane (delegate `OnComponentBeginOverlap_Event_0`))
    (`KismetSystemLibrary.PrintString` "collide w slicemesh")
    (`/Engine/EditorBlueprintResources/StandardMacros.DoOnce` false :!label _label
      (:`Completed`
        (bind _asprocedural_mesh_component (cast `ProceduralMeshComponent` (stale `OnComponentBeginOverlap_Event_0` OtherComp)))
        (bind _outotherhalfprocmesh (`KismetProceduralMeshLibrary.SliceProceduralMesh` _asprocedural_mesh_component _returnvalue (`SceneComponent.GetUpVector` _plane) true "CreateNewSectionForCap" "/Game/Game/Mesh/Monster/Monster_Gloem_Mesh/Gloem_RedBlu.Gloem_RedBlu"))
        (`PrimitiveComponent.SetSimulatePhysics` _outotherhalfprocmesh true)
        (`PrimitiveComponent.AddRadialImpulse` _asprocedural_mesh_component _returnvalue 300.0 500.0 "RIF_Constant" true)))
    (else
      (set `self.CanCut` false)
      (goto _label :!via `Reset`))))

(event `OnComponentBeginOverlap_Event_0`
  (params (OverlappedComponent :type "PrimitiveComponent Object Reference") (OtherActor :type "Actor Object Reference") (OtherComp :type "PrimitiveComponent Object Reference") (OtherBodyIndex :type Integer) (bFromSweep :type Boolean) (SweepResult :type "HitResult Structure (by ref)")))

(fn `UserConstructionScript`)