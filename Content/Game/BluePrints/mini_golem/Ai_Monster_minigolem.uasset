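; AI controller for the mini golem monster that wanders on duty and switches to combat when it sights an enemy.
; Patrol repeatedly picks random nearby points, and a gated move retries failures via reachable points, stepping toward distant targets.
; Sighting locks on, approaches, enables attack mode after a delay and temporarily mutes senses.
; A timer loop resumes patrol once alerts go stale; hearing checks teams but takes no action.
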(event `self.ReceiveBeginPlay`
  (set `self.Ch` (`self.K2_GetPawn`))
  (`/Game/Game/Interface/BPI_Ai.ResumeDuty`))

(event `/Game/Game/Interface/BPI_Ai.GoToLocation`
  (params (Targetlocation :type "Vector Structure"))
  (bind _randomlocation (`self.Get TargetLocation` Targetlocation))
  (bind _output_get (set `self.Destination` Targetlocation))
  (`/Engine/EditorBlueprintResources/StandardMacros.DoOnce` false :!label _label
    (:`Completed`
      (`|AIMoveTo` null _output_get null
        (:`OnSuccess`
          (goto _label :!via `Reset`))
        (:`OnFail`
          (`|AIMoveTo` null _randomlocation null 200.0 :!label _label_2
            (:`OnSuccess`
              (if (< (`self.Get Distance And Direction` _randomlocation (`self.K2_GetActorLocation` (`self.Ch`))) 200.0)
                (goto _label :!via `Reset`)
                (else
                  _)))
            (:`OnFail`
              _))
          (`KismetSystemLibrary.Delay` 0.4)
          (goto _label_2))))))

(event `/Game/Game/Interface/BPI_Ai.ResumeDuty`
  (bind _ch (`self.Ch`))
  (set `self.Seen` false)
  (message `/Game/Game/Interface/BPI_Character.ToggleRun` _ch false)
  (message `/Game/Game/Interface/BPI_Character.ToggleSprint` _ch false)
  (`/Game/Game/Interface/BPI_Ai.GoToLocation` (`NavigationSystemV1.K2_GetRandomReachablePointInRadius` (`self.K2_GetActorLocation` _ch) 1000.0 null null) :!label _label_3)
  (`KismetSystemLibrary.Delay` (`KismetMathLibrary.RandomFloatInRange` 5.0 10.0))
  (bind _reaction (`/Game/Game/Interface/BPI_Ai.OnReaction_AI`))
  (if (not _reaction)
    (goto _label_3)))

(fn `Get Distance And Direction`
  (params (`Target Location` :type "Vector Structure") (`Currect Location` :type "Vector Structure"))
  (returns (Distance :type "Float (double-precision)") (Direction :type "Vector Structure"))
  (bind _returnvalue (- `Target Location` `Currect Location`))
  (return (`KismetMathLibrary.VSize` _returnvalue) (`KismetMathLibrary.Normal` _returnvalue 0.0)))

(fn `Get TargetLocation`
  (params (terget :type "Vector Structure (by ref)"))
  (returns (RandomLocation :type "Vector Structure"))
  (bind _randomlocation (`NavigationSystemV1.K2_GetRandomReachablePointInRadius` terget 100.0 null null))
  (bind _returnvalue (`self.K2_GetActorLocation` (`self.Ch`)))
  (bind (_distance _direction) (`self.Get Distance And Direction` _randomlocation _returnvalue))
  (if (< _distance 2500.0)
    (return _randomlocation)
    (else
      (return (`NavigationSystemV1.K2_GetRandomReachablePointInRadius` (+ _returnvalue (* _direction 1500.0)) 100.0 null null)))))

(fn `OnReaction_AI`
  (returns (Reaction :type Boolean))
  (return (`self.Seen`)))

(fn `UserConstructionScript`)