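; Mini golem enemy Character: a melee fighter with a health widget, team checks, blocking, hit reactions and knockback.
; Attack mode locks on and alternates timed attack phases with strafing and random blocking, using the target's under-attack flag to stagger attackers.
; Attacks play random montages and briefly enable hit capsules; CheckHit applies range, block and dodge rules.
; Incoming hammer or sword damage reduces health; death triggers ragdoll, player HP recovery and an apple pickup drop.
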(event `self.ReceiveBeginPlay`
  (set `self.ServerDamage` (`self.DMG`))
  (set `self.ServerRecovery` (`self.Recovery`))
  (set `self.anim` (`SkeletalMeshComponent.GetAnimInstance` (`self.Mesh`)))
  (`self.UpdateActorDetails`))

(event `SetunderAttack`
  (params (Duration :type "Float (double-precision)" :default 0.5))
  (set `self.under Attack` true)
  (`KismetSystemLibrary.Delay` Duration)
  (set `self.under Attack` false))

(event `self.ReceiveTick`
  (params (DeltaSeconds :type "Float (single-precision)"))
  (bind (_returnvalue_roll _returnvalue_pitch) (`KismetMathLibrary.BreakRotator` (`self.K2_GetActorRotation`)))
  (bind _lolcked_enemy (`self.lolcked enemy`))
  (bind _returnvalue (< (`self.GetDistanceTo` _lolcked_enemy self) (`self.Lock distance`)))
  (bind _returnvalue_2 (`KismetMathLibrary.MakeRotator` 0.0 0.0 (.yaw (`self.GetControlRotation`))))
  (bind (_returnvalue_roll_2 _returnvalue_pitch_2 _returnvalue_yaw) (`KismetMathLibrary.BreakRotator` (`KismetMathLibrary.RInterpTo` (`self.K2_GetActorRotation`) (`KismetMathLibrary.FindLookAtRotation` (`self.K2_GetActorLocation`) (`self.K2_GetActorLocation` _lolcked_enemy)) 0.5 0.2)))
  (set `self.Health` (`self.Health`))
  (set `self.ready_cpp` (`self.ready`))
  (if (and (`self.lockedOn`) (not (`self.dodging`)))
    (`/Engine/EditorBlueprintResources/StandardMacros.IsValid` _lolcked_enemy
      (:`Is Valid`
        (set `CharacterMovementComponent.bOrientRotationToMovement` (not _returnvalue) (`self.CharacterMovement`))
        (if _returnvalue
          (`self.K2_SetActorRotation` (`KismetMathLibrary.MakeRotator` _returnvalue_roll _returnvalue_pitch _returnvalue_yaw))))
      (:`Is Not Valid`
        _)))
  (`self.UpdateActorDetails`)
  (`/Engine/EditorBlueprintResources/StandardMacros.IsValid` (`self.lolcked enemy`)
    (:`Is Valid`
      (if (not (`self.Attacking`))
        (`self.AddMovementInput` (`KismetMathLibrary.GetRightVector` _returnvalue_2) (`self.FightStrafe`))
        (`self.AddMovementInput` (`KismetMathLibrary.GetForwardVector` _returnvalue_2) (select `bool` (> (`self.GetDistanceTo` (`self.lolcked enemy`) self) 500.0) :`false` -1.0 :`true` 1.0 :!type "Float (single-precision)"))))))

(event `self.UpdateActorDetails`
  (bind _widget (`self.Widget`))
  (`SceneComponent.SetHiddenInGame` _widget (not (`self.in Attack mode`)) false)
  (message `/Game/Game/Interface/BPI_UI.UpdateProgress` (`WidgetComponent.GetUserWidgetObject` _widget) (/ (`self.Health`) (`self.Health_MAX`))))

(event `InputAxis|MoveForward` :overrideparent false
  (params (AxisValue :type "Float (single-precision)"))
  ;[1 1 1] 코멘트
  (if (`self.canMove`)
    (`self.AddMovementInput` (`KismetMathLibrary.GetForwardVector` (`KismetMathLibrary.MakeRotator` 0.0 0.0 (.yaw (`self.GetControlRotation`)))) AxisValue)))

(event `self.ToggleMovement`
  (params (`Enable/Disable` :type Boolean))
  ;[1 1 1] 코멘트
  (bind _output_get (set `self.canMove` `Enable/Disable`))
  (set `self.ready` _output_get))

(event `InputAxis|MoveRight` :overrideparent false
  (params (AxisValue :type "Float (single-precision)"))
  ;[1 1 1] 코멘트
  (if true
    (`self.AddMovementInput` (`KismetMathLibrary.GetRightVector` (`KismetMathLibrary.MakeRotator` 0.0 0.0 (.yaw (`self.GetControlRotation`)))) (+ AxisValue (`self.FightStrafe`)))))

(event `self.ToggleRun`
  (params (enable :type Boolean))
  (bind _charactermovement (`self.CharacterMovement`))
  (bind _output_get (set `self.Running` enable))
  (if _output_get
    (set `CharacterMovementComponent.MaxWalkSpeed` (`self.walkingSpeed`) _charactermovement)
    (else
      (set `CharacterMovementComponent.MaxWalkSpeed` (`self.RunningSpeed`) _charactermovement))))

(event `self.ToggleSprint`
  (params (enable :type Boolean))
  (if enable
    (set `self.sprinting` true)
    (`self.ToggleRun` true)
    (set `CharacterMovementComponent.MaxWalkSpeed` 800.0 (`self.CharacterMovement`))))

(event `self.ToggleBlock`
  (params (enable :type Boolean))
  (if enable
    (set `self.Blocking` true)
    (if (`self.Blocking`)
      (`self.PlayAnimMontage` "/Game/Game/Mesh/Monster/Ice_Spirit/Ice_Spirit_Animation/Ice_Spirit_Block_Montage.Ice_Spirit_Block_Montage" 1.6)
      (`/Engine/EditorBlueprintResources/StandardMacros.DoOnce` false :!label _label
        (:`Completed`
          (`|ExecutionSequence`
            (:`then_0`
              (bind _closestenemy (`self.Get Closest Enemy`))
              (`/Engine/EditorBlueprintResources/StandardMacros.IsValid` _closestenemy
                (:`Is Valid`
                  (`self.Lockon` _closestenemy true)
                  (`KismetSystemLibrary.Delay` 1.5)
                  (if (not (`self.Blocking`))
                    (goto _label :!via `Reset`)))))
            (:`then_1`
              (`KismetSystemLibrary.Delay` 0.5))))))
    (else
      (set `self.Blocking` false)
      (`self.StopAnimMontage` null))))

(event `self.Lockon`
  (params (`locked enemy` :type "Actor Object Reference") (`lock on/off` :type Boolean))
  (if true
    (`/Engine/EditorBlueprintResources/StandardMacros.IsValid` `locked enemy`
      (:`Is Valid`
        (set `self.lolcked enemy` `locked enemy`)
        (set `self.lockedOn` true)
        (set `CharacterMovementComponent.bOrientRotationToMovement` false (`self.CharacterMovement`))))
    (else
      (set `self.lockedOn` false)
      (set `CharacterMovementComponent.bOrientRotationToMovement` true (`self.CharacterMovement`)))))

(event `self.ToggleAttacking`
  (params (enable :type Boolean) (player :type "Actor Object Reference"))
  (bind _returnvalue (`self.K2_GetActorLocation` player))
  (bind _output_get (set `self.Attacking` enable))
  (if _output_get
    (`/Engine/EditorBlueprintResources/StandardMacros.DoOnce` false :!label _label_2
      (:`Completed`
        (`/Engine/EditorBlueprintResources/StandardMacros.IsValid` player :!label _label_3
          (:`Is Valid`
            (if (< (`self.GetDistanceTo` player self) (`self.hitRange`)) :!label _label_4
              (bind _under_attack (message `/Game/Game/Interface/BPI_Character.isunderAttack` player 0.5))
              (if _under_attack
                (`self.minigolem AI Attack`))
              (`KismetSystemLibrary.Delay` (`KismetMathLibrary.RandomFloatInRange` 1.0 4.0))
              (if (`self.Attacking`)
                (goto _label_3)
                (else
                  (goto _label_2 :!via `Reset`)))
              (else
                (`AIBlueprintHelperLibrary.SimpleMoveToLocation` (`AIBlueprintHelperLibrary.GetAIController` self) (+ (* (`KismetMathLibrary.Normal` (- (`self.K2_GetActorLocation`) _returnvalue)) (* (`self.hitRange`) 0.6)) _returnvalue))
                (`KismetSystemLibrary.Delay` 2.0)
                (goto _label_4)))))))))

(event `self.ToggleAttackMode`
  (params (enable :type Boolean) (enemy :type "Actor Object Reference"))
  (bind _lolcked_enemy (`self.lolcked enemy`))
  (bind _output_get (set `self.in Attack mode` enable))
  (if _output_get
    (`self.Lockon` enemy true)
    (`/Engine/EditorBlueprintResources/StandardMacros.DoOnce` false
      (:`Completed`
        (`/Engine/EditorBlueprintResources/StandardMacros.FlipFlop` :!label _label_5
          (:`A`
            (set `self.FightStrafe` 0.0)
            (`self.ToggleAttacking` true _lolcked_enemy)
            (`KismetSystemLibrary.Delay` (`KismetMathLibrary.RandomFloatInRange` 6.0 10.0)))
          (:`B`
            (`self.ToggleBlock` (`KismetMathLibrary.RandomBool`))
            (set `self.FightStrafe` (`KismetMathLibrary.RandomFloatInRange` -0.5 0.5))
            (`self.ToggleAttacking` false _lolcked_enemy)
            (`KismetSystemLibrary.Delay` (`KismetMathLibrary.RandomFloatInRange` 4.0 8.0))))
        (if (`self.in Attack mode`)
          (goto _label_5))))
    (else
      (`self.ToggleAttacking` false)
      (`self.Lockon` null))))

(event `self.minigolem AI Attack`
  (bind _returnvalue (`KismetMathLibrary.RandomInteger` 2))
  (bind _capsule (`self.Capsule`))
  (if (not (`self.Is Dead`))
    (`/Engine/EditorBlueprintResources/StandardMacros.DoOnce` false :!label _label_6
      (:`Completed`
        (if (`self.lockedOn`)
          (set `self.RandAttack` _returnvalue :!label _label_7)
          (`self.PlayAnimMontage` (select `int` _returnvalue :`0` "/Game/Game/Mesh/Monster/Ice_Spirit/Ice_Spirit_Animation/Ice_Spirit_Attack_Anim_Montage.Ice_Spirit_Attack_Anim_Montage" :`1` "/Game/Game/Mesh/Monster/Ice_Spirit/Ice_Spirit_Animation/Ice_Spirit_Attack2_Anim_Montage.Ice_Spirit_Attack2_Anim_Montage" :`2` "/Game/Game/Mesh/Monster/Ice_Spirit/Ice_Spirit_Animation/Ice_Spirit_Attack2_Anim_Montage.Ice_Spirit_Attack2_Anim_Montage" :!type "AnimMontage Object Reference") 1.6)
          (`|ExecutionSequence`
            (:`then_0`
              (goto _label_6 :!via `Reset`))
            (:`then_1`
              (`PrimitiveComponent.SetCollisionEnabled` _capsule "QueryAndPhysics")
              (`PrimitiveComponent.SetCollisionEnabled` (`self.Capsule1`) "QueryAndPhysics")
              (`KismetSystemLibrary.Delay` 0.4)
              (`PrimitiveComponent.SetCollisionEnabled` _capsule "NoCollision")
              (`PrimitiveComponent.SetCollisionEnabled` (`self.Capsule1`) "NoCollision")))
          (else
            (bind _closestenemy (`self.Get Closest Enemy`))
            (set `self.lolcked enemy` _closestenemy)
            (`/Engine/EditorBlueprintResources/StandardMacros.IsValid` _closestenemy
              (:`Is Valid`
                (`|ExecutionSequence`
                  (:`then_0`
                    (goto _label_7))
                  (:`then_1`
                    (`self.RotateToActor` _closestenemy))))
              (:`Is Not Valid`
                (goto _label_7)))))))))

(event `self.CheckHit`
  (params (`Can Block` :type Boolean))
  (bind _closestenemy (`self.closestEnemy`))
  (bind _closestenemy_2 (`self.closestEnemy`))
  (`/Engine/EditorBlueprintResources/StandardMacros.IsValid` _closestenemy
    (:`Is Valid`
      _)
    (:`Is Not Valid`
      (`self.Get Closest Enemy`)))
  (if (< (`KismetMathLibrary.VSize` (- (`SceneComponent.GetSocketLocation` (`self.Capsule`) "None") (`self.K2_GetActorLocation` (`self.closestEnemy`)))) (`self.hitRange`))
    (bind _team_number (message `/Game/Game/Interface/BPI_Character.GetTeam` _closestenemy))
    (if (== _team_number -1)
      (bind (_blocking _dodging) (message `/Game/Game/Interface/BPI_Character.isBlockingOrDodging` _closestenemy))
      (if (not _dodging)
        (if _blocking
          (`GameplayStatics.PlaySoundAtLocation` "/Game/Game/Sound/player/Block.Block" (`self.K2_GetActorLocation` _closestenemy_2) (struct) 1.0 1.0 0.0 null null null)
          (`GameplayStatics.SpawnEmitterAtLocation` null)
          (message `/Game/Game/Interface/BPI_Character.Counter` _closestenemy_2)
          (else
            (message `/Game/Game/Interface/BPI_Character.ToggleBlock` _closestenemy_2 false)
            (`GameplayStatics.PlaySoundAtLocation` "/Game/Game/Sound/player/Armor_MetalHit_00.Armor_MetalHit_00" (`self.K2_GetActorLocation`) (struct) 1.0 1.0 0.0 null null null)))
        (message `/Game/Game/Interface/BPI_Damageable.OnweaponHit player` _closestenemy_2 self (`self.DMG`))))))

(event `/Game/Game/Interface/BPI_Damageable.OnWeaponHit MiniGolem`
  (params (`Source Weapon Hit` :type "Actor Object Reference") (`HIt Location` :type "Vector Structure") (KnockBack :type Boolean))
  (bind _returnvalue (`self.K2_GetActorLocation`))
  (bind _returnvalue_2 (`self.K2_GetActorLocation` `Source Weapon Hit`))
  (bind (_returnvalue_roll _returnvalue_pitch _returnvalue_yaw) (`KismetMathLibrary.BreakRotator` (`KismetMathLibrary.FindLookAtRotation` _returnvalue _returnvalue_2)))
  (bind _yes_no (message `/Game/Game/Interface/BPI_Character.isEnemy` `Source Weapon Hit` (`self.team`)))
  (if _yes_no
    (if (`self.dodging`)
      _
      (elif KnockBack
        (`self.PlayAnimMontage` "/Game/Game/Mesh/Monster/Ice_Spirit/Ice_Spirit_Animation/Ice_Spirit_Konck_Back_Montage.Ice_Spirit_Konck_Back_Montage")
        (`KismetSystemLibrary.MoveComponentTo` (`self.CapsuleComponent`) (+ _returnvalue_2 (* (`KismetMathLibrary.Normal` (- _returnvalue _returnvalue_2)) 300.0)) (`KismetMathLibrary.MakeRotator` 0.0 0.0 _returnvalue_yaw) false false 0.1)
        (elif (`self.Blocking`)
          (`self.PlayAnimMontage` "/Game/Game/Mesh/Monster/Ice_Spirit/Ice_Spirit_Animation/Ice_Spirit_Hit_Montage.Ice_Spirit_Hit_Montage")
          (`|ExecutionSequence`
            (:`then_0`
              (`KismetSystemLibrary.Delay` 0.2)
              (if (not (`self.Blocking`))
                (`self.PlayAnimMontage` "/Game/Game/Mesh/Monster/Ice_Spirit/Ice_Spirit_Animation/Ice_Spirit_Release_Block_Montage.Ice_Spirit_Release_Block_Montage")))
            (:`then_1`
              (`KismetSystemLibrary.Delay` 0.3 :!label _label_8)
              (`self.RotateToActor` `Source Weapon Hit`)))
          (else
            (`self.PlayAnimMontage` "/Game/Game/Mesh/Monster/Ice_Spirit/Ice_Spirit_Animation/Ice_Spirit_Hit_Montage.Ice_Spirit_Hit_Montage")
            (`CharacterMovementComponent.AddImpulse` (`self.CharacterMovement`) (* (`self.GetActorForwardVector` self) -500.0) true)
            (bind (_currenthammer _hammer) (message `/Game/Game/Interface/BPI_Character.GetHammer` `Source Weapon Hit`))
            (if _hammer
              (bind _dmg (message `/Game/Game/Interface/BPI_weapon.GetDamge` _currenthammer))
              (`self.UpdateHealth` _dmg `Source Weapon Hit`
                (:`True`
                  _))
              (else
                (bind _currentsword (message `/Game/Game/Interface/BPI_Character.GetSword` `Source Weapon Hit`))
                (bind _dmg_2 (message `/Game/Game/Interface/BPI_weapon.GetDamge` _currentsword))
                (`self.UpdateHealth` _dmg_2 `Source Weapon Hit`
                  (:`True`
                    _))))
            (`GameplayStatics.PlaySoundAtLocation` null (`self.K2_GetActorLocation`) (struct) 1.0 1.0 0.0 null null null)
            (goto _label_8)))))))

(fn `Get Closest Enemy`
  (returns (closestEnemy :type "Actor Object Reference"))
  (bind _returnvalue (`self.K2_GetActorLocation`))
  (set `self.closestEnemy` null)
  (bind _outhits (`KismetSystemLibrary.SphereTraceMultiForObjects` _returnvalue _returnvalue 1000.0 (`|MakeArray` "ObjectTypeQuery7" :!type "EObjectTypeQuery Enum")))
  (for _array_element _outhits
    (bind _yes_no (message `/Game/Game/Interface/BPI_Character.isEnemy` (`.HitActor` (`GameplayStatics.BreakHitResult` _array_element)) (`self.team`)))
    (if _yes_no
      (`/Engine/EditorBlueprintResources/StandardMacros.IsValid` (`self.closestEnemy`)
        (:`Is Valid`
          (if (not (< (`self.GetDistanceTo` (`self.closestEnemy`) self) (`self.GetDistanceTo` (`.HitActor` (`GameplayStatics.BreakHitResult` _array_element)) self)))
            (set `self.closestEnemy` (`.HitActor` (`GameplayStatics.BreakHitResult` _array_element)) :!label _label)))
        (:`Is Not Valid`
          (goto _label)))))
  (return (`self.closestEnemy`)))

(fn `GetHammer`
  (returns (CurrentHammer :type "Actor Object Reference") (Hammer :type Boolean))
  (return null false))

(fn `GetSword`
  (returns (CurrentSword :type "Actor Object Reference") (Sword :type Boolean))
  (return null false))

(fn `GetTeam`
  (returns (`team number` :type Integer))
  (return (`self.Team`)))

(fn `Is Dead`
  (returns (Dead :type Boolean))
  (return (<= (`self.Health`) 0.0)))

(fn `isBlockingOrDodging`
  (returns (blocking :type Boolean) (dodging :type Boolean))
  (return (`self.Blocking`) (`self.dodging`)))

(fn `isEnemy`
  (params (`team number` :type Integer))
  (returns (`yes/no` :type Boolean))
  (return (and (!= `team number` (`self.Team`)) (not (`self.Is Dead`)))))

(fn `isunderAttack`
  (params (`Attack Duration` :type "Float (double-precision)"))
  (returns (`under Attack` :type Boolean))
  (if (`self.under Attack`)
    (return true)
    (else
      (`self.SetunderAttack` `Attack Duration`)
      (return false))))

(fn `ON_Reaction`
  (returns (Reaction :type Boolean))
  (bind _reaction (message `/Game/Game/Interface/BPI_Ai.OnReaction_AI` (`self.GetController`)))
  (return _reaction))

(fn `UserConstructionScript`)