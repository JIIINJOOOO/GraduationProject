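; Melee AI monster character (mini golem folder, goblin animations) that locks onto enemies of other teams and fights them.
; Attack mode alternates timed attack phases with strafing and random blocking; attacks first claim the player's under-attack window, spacing out attackers.
; Weapon hits trigger block, hit or knockback reactions via interface messages and update health and its widget.
; Death ragdolls the body, notifies the killer, sends HP recovery and spawns an apple pickup.
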(event `ChangeDamageColor`
  ;[1 1 1] ChangeDamageColor_Event
  (`PrimitiveComponent.SetMaterial` (`self.Mesh`) 0 "/Game/Game/Mesh/Monster/Monster_Goblin_Mesh/phong1_Inst.phong1_Inst")
  (`KismetSystemLibrary.Delay` 0.2)
  (`PrimitiveComponent.SetMaterial` (`self.Mesh`) 0 "/Game/Game/Mesh/Monster/Monster_Goblin_Mesh/phong1.phong1"))

(event `self.ReceiveBeginPlay`
  (set `self.anim` (`SkeletalMeshComponent.GetAnimInstance` (`self.Mesh`)))
  (`/Game/Game/Interface/BPI_Character.UpdateActorDetails`))

(event `SetunderAttack`
  (params (Duration :type "Float (double-precision)" :default 0.5))
  (set `self.under Attack` true)
  (`KismetSystemLibrary.Delay` Duration)
  (set `self.under Attack` false))

(event `self.ReceiveTick`
  (params (DeltaSeconds :type "Float (single-precision)"))
  (bind (_returnvalue_roll _returnvalue_pitch) (`KismetMathLibrary.BreakRotator` (`self.K2_GetActorRotation`)))
  (bind _lolcked_enemy (`self.lolcked enemy`))
  (bind _returnvalue (< (`self.GetDistanceTo` _lolcked_enemy self) (`self.Lock distance`)))
  (bind _returnvalue_2 (`KismetMathLibrary.MakeRotator` 0.0 0.0 (.yaw (`self.GetControlRotation`))))
  (bind (_returnvalue_roll_2 _returnvalue_pitch_2 _returnvalue_yaw) (`KismetMathLibrary.BreakRotator` (`KismetMathLibrary.RInterpTo` (`self.K2_GetActorRotation`) (`KismetMathLibrary.FindLookAtRotation` (`self.K2_GetActorLocation`) (`self.K2_GetActorLocation` _lolcked_enemy)) 0.5 0.2)))
  (set `self.IsAttacking_cpp` (`self.Attacking`))
  (set `self.IsBlocking_cpp` (`self.Blocking`))
  (set `self.IsDodging_cpp` (`self.dodging`))
  (if (and (`self.lockedOn`) (not (`self.dodging`)))
    (`/Engine/EditorBlueprintResources/StandardMacros.IsValid` _lolcked_enemy
      (:`Is Valid`
        (set `CharacterMovementComponent.bOrientRotationToMovement` (not _returnvalue) (`self.CharacterMovement`))
        (if _returnvalue
          (`self.K2_SetActorRotation` (`KismetMathLibrary.MakeRotator` _returnvalue_roll _returnvalue_pitch _returnvalue_yaw))))
      (:`Is Not Valid`
        _)))
  (`/Engine/EditorBlueprintResources/StandardMacros.IsValid` (`self.lolcked enemy`)
    (:`Is Valid`
      (if (not (`self.Attacking`))
        (`self.AddMovementInput` (`KismetMathLibrary.GetRightVector` _returnvalue_2) (`self.FightStrafe`))
        (`self.AddMovementInput` (`KismetMathLibrary.GetForwardVector` _returnvalue_2) (select `bool` (> (`self.GetDistanceTo` (`self.lolcked enemy`) self) 500.0) :`false` -1.0 :`true` 1.0 :!type "Float (single-precision)"))))))

(event `/Game/Game/Interface/BPI_Character.UpdateActorDetails`
  (bind _widget (`self.Widget`))
  (`SceneComponent.SetHiddenInGame` _widget (not (`self.in Attack mode`)) false)
  (message `/Game/Game/Interface/BPI_UI.UpdateProgress` (`WidgetComponent.GetUserWidgetObject` _widget) (/ (`self.Health`) (`self.Health_MAX`))))

(event `InputAxis|MoveForward` :overrideparent false
  (params (AxisValue :type "Float (single-precision)"))
  ;[1 1 1] 코멘트
  (if (`self.canMove`)
    (`self.AddMovementInput` (`KismetMathLibrary.GetForwardVector` (`KismetMathLibrary.MakeRotator` 0.0 0.0 (.yaw (`self.GetControlRotation`)))) AxisValue)))

(event `/Game/Game/Interface/BPI_Character.ToggleMovement`
  (params (`Enable/Disable` :type Boolean))
  ;[1 1 1] 코멘트
  (bind _output_get (set `self.canMove` `Enable/Disable`))
  (set `self.ready` _output_get))

(event `InputAxis|MoveRight` :overrideparent false
  (params (AxisValue :type "Float (single-precision)"))
  ;[1 1 1] 코멘트
  (if true
    (`self.AddMovementInput` (`KismetMathLibrary.GetRightVector` (`KismetMathLibrary.MakeRotator` 0.0 0.0 (.yaw (`self.GetControlRotation`)))) (+ AxisValue (`self.FightStrafe`)))))

(event `/Game/Game/Interface/BPI_Character.ToggleRun`
  (params (enable :type Boolean))
  (bind _charactermovement (`self.CharacterMovement`))
  (bind _output_get (set `self.Running` enable))
  (if _output_get
    (set `CharacterMovementComponent.MaxWalkSpeed` (`self.walkingSpeed`) _charactermovement)
    (else
      (set `CharacterMovementComponent.MaxWalkSpeed` (`self.RunningSpeed`) _charactermovement))))

(event `/Game/Game/Interface/BPI_Character.ToggleSprint`
  (params (enable :type Boolean))
  (if enable
    (set `self.sprinting` true)
    (`/Game/Game/Interface/BPI_Character.ToggleRun` true)
    (set `CharacterMovementComponent.MaxWalkSpeed` 800.0 (`self.CharacterMovement`))))

(event `/Game/Game/Interface/BPI_Character.ToggleBlock`
  (params (enable :type Boolean))
  (if enable
    (set `self.Blocking` true)
    (if (`self.Blocking`)
      (`self.PlayAnimMontage` "/Game/Game/Mesh/Monster/Monster_Goblin_Mesh/Animations/Standing_Block_Idle_mixamo_com_Montage.Standing_Block_Idle_mixamo_com_Montage" 1.6)
      (`/Engine/EditorBlueprintResources/StandardMacros.DoOnce` false :!label _label
        (:`Completed`
          (`|ExecutionSequence`
            (:`then_0`
              (bind _closestenemy (`self.Get Closest Enemy`))
              (`/Engine/EditorBlueprintResources/StandardMacros.IsValid` _closestenemy
                (:`Is Valid`
                  (`/Game/Game/Interface/BPI_Character.Lockon` _closestenemy true)
                  (`/Game/Game/Interface/BPI_Character.Attack Move` 500.0)
                  (`KismetSystemLibrary.Delay` 1.5)
                  (if (not (`self.Blocking`))
                    (goto _label :!via `Reset`)))))
            (:`then_1`
              (`KismetSystemLibrary.Delay` 0.5))))))
    (else
      (set `self.Blocking` false)
      (`self.StopAnimMontage` null))))

(event `/Game/Game/Interface/BPI_Character.Lockon`
  (params (`locked enemy` :type "Actor Object Reference") (`lock on/off` :type Boolean))
  (if true
    (`/Engine/EditorBlueprintResources/StandardMacros.IsValid` `locked enemy`
      (:`Is Valid`
        (set `self.lolcked enemy` `locked enemy`)
        (set `self.lockedOn` true)
        (set `CharacterMovementComponent.bOrientRotationToMovement` false (`self.CharacterMovement`)))
      (:`Is Not Valid`
        (bind _closestenemy (`self.Get Closest Enemy`))
        (`/Engine/EditorBlueprintResources/StandardMacros.IsValid` _closestenemy
          (:`Is Valid`
            (`/Game/Game/Interface/BPI_Character.Lockon` _closestenemy true))
          (:`Is Not Valid`
            (set `self.lockedOn` false)))))
    (else
      (set `self.lockedOn` false)
      (set `CharacterMovementComponent.bOrientRotationToMovement` true (`self.CharacterMovement`)))))

(event `/Game/Game/Interface/BPI_Character.Gobin AI Attack`
  (if (not (`self.Is Dead`))
    (`/Engine/EditorBlueprintResources/StandardMacros.DoOnce` false :!label _label_2
      (:`Completed`
        (if (`self.lockedOn`)
          (bind _output_get (set `self.RandAttack` (`KismetMathLibrary.RandomInteger` 3) :!label _label_3))
          (`self.PlayAnimMontage` (select `int` _output_get :`0` "/Game/Game/Mesh/Monster/Monster_Goblin_Mesh/AnimMontage/Golblin_slash_Montage.Golblin_slash_Montage" :`1` "/Game/Game/Mesh/Monster/Monster_Goblin_Mesh/Animations/Goblin_Melee_Attack_Backhand_mixamo_com_Montage.Goblin_Melee_Attack_Backhand_mixamo_com_Montage" :`2` "/Game/Game/Mesh/Monster/Monster_Goblin_Mesh/Animations/Goblin_Melee_Attack_Downward_mixamo_com_Montage.Goblin_Melee_Attack_Downward_mixamo_com_Montage" :`3` "/Game/Game/Mesh/Monster/Monster_Goblin_Mesh/Animations/Goblin_Melee_Combo_Attack_Ver__3_mixamo_com_Montage.Goblin_Melee_Combo_Attack_Ver__3_mixamo_com_Montage" :!type "AnimMontage Object Reference") 1.6)
          (`|ExecutionSequence`
            (:`then_0`
              (goto _label_2 :!via `Reset`)))
          (else
            (bind _closestenemy (`self.Get Closest Enemy`))
            (set `self.lolcked enemy` _closestenemy)
            (`/Engine/EditorBlueprintResources/StandardMacros.IsValid` _closestenemy
              (:`Is Valid`
                (`|ExecutionSequence`
                  (:`then_0`
                    (goto _label_3))
                  (:`then_1`
                    (`self.RotateToActor` _closestenemy))))
              (:`Is Not Valid`
                (goto _label_3)))))))))

(event `/Game/Game/Interface/BPI_Character.CheckHit`
  (params (`Can Block` :type Boolean))
  (bind _closestenemy (`self.closestEnemy`))
  (bind _closestenemy_2 (`self.closestEnemy`))
  (`/Engine/EditorBlueprintResources/StandardMacros.IsValid` _closestenemy
    (:`Is Valid`
      _)
    (:`Is Not Valid`
      (`self.Get Closest Enemy`)))
  (if (< (`KismetMathLibrary.VSize` (- (0.0 0.0 0.0) (`self.K2_GetActorLocation` (`self.closestEnemy`)))) (`self.hitRange`))
    (bind _team_number (message `/Game/Game/Interface/BPI_Character.GetTeam` _closestenemy))
    (if (== _team_number -1)
      (bind (_blocking _dodging) (message `/Game/Game/Interface/BPI_Character.isBlockingOrDodging` _closestenemy))
      (if _blocking
        (message `/Game/Game/Interface/BPI_Character.updateStamina` _closestenemy_2 (`self.DMG`))
        (`GameplayStatics.PlaySoundAtLocation` "/Game/StarterContent/Audio/Collapse01.Collapse01" (`self.K2_GetActorLocation` _closestenemy_2) (struct) 1.0 1.0 0.0 null null null)
        (`GameplayStatics.SpawnEmitterAtLocation` null)
        (message `/Game/Game/Interface/BPI_Character.Counter` _closestenemy_2)
        (else
          (message `/Game/Game/Interface/BPI_Character.ToggleBlock` _closestenemy_2 false)
          (`GameplayStatics.PlaySoundAtLocation` null (`self.K2_GetActorLocation`) (struct) 1.0 1.0 0.0 null null null)))
      (message `/Game/Game/Interface/BPI_Damageable.OnweaponHit player` _closestenemy_2 self (`self.DMG`)))))

(event `/Game/Game/Interface/BPI_Character.ToggleAttacking`
  (params (enable :type Boolean) (player :type "Actor Object Reference"))
  (bind _returnvalue (`self.K2_GetActorLocation` player))
  (bind _output_get (set `self.Attacking` enable))
  (if _output_get
    (`/Engine/EditorBlueprintResources/StandardMacros.DoOnce` false :!label _label_4
      (:`Completed`
        (`/Engine/EditorBlueprintResources/StandardMacros.IsValid` player :!label _label_5
          (:`Is Valid`
            (if (< (`self.GetDistanceTo` player self) (`self.hitRange`)) :!label _label_6
              (bind _under_attack (message `/Game/Game/Interface/BPI_Character.isunderAttack` player 0.5))
              (if _under_attack
                (`/Game/Game/Interface/BPI_Character.Gobin AI Attack`))
              (`KismetSystemLibrary.Delay` (`KismetMathLibrary.RandomFloatInRange` 1.0 3.0))
              (if (and (`self.Attacking`) (not (`self.Is Dead`)))
                (goto _label_5)
                (else
                  (goto _label_4 :!via `Reset`)))
              (else
                (`AIBlueprintHelperLibrary.SimpleMoveToLocation` (`AIBlueprintHelperLibrary.GetAIController` self) (+ (* (`KismetMathLibrary.Normal` (- (`self.K2_GetActorLocation`) _returnvalue)) (* (`self.hitRange`) 0.6)) _returnvalue))
                (`KismetSystemLibrary.Delay` 2.0)
                (goto _label_6)))))))))

(event `/Game/Game/Interface/BPI_Character.ToggleAttackMode`
  (params (enable :type Boolean) (enemy :type "Actor Object Reference"))
  (bind _lolcked_enemy (`self.lolcked enemy`))
  (bind _output_get (set `self.in Attack mode` enable))
  (`/Game/Game/Interface/BPI_Character.UpdateActorDetails`)
  (if _output_get
    (`/Game/Game/Interface/BPI_Character.Lockon` enemy true)
    (`/Engine/EditorBlueprintResources/StandardMacros.DoOnce` false
      (:`Completed`
        (`/Engine/EditorBlueprintResources/StandardMacros.FlipFlop` :!label _label_7
          (:`A`
            (set `self.FightStrafe` 0.0)
            (`/Game/Game/Interface/BPI_Character.ToggleAttacking` true _lolcked_enemy)
            (`KismetSystemLibrary.Delay` (`KismetMathLibrary.RandomFloatInRange` 5.0 9.0)))
          (:`B`
            (`/Game/Game/Interface/BPI_Character.ToggleBlock` (`KismetMathLibrary.RandomBool`))
            (set `self.FightStrafe` (`KismetMathLibrary.RandomFloatInRange` -0.5 0.5))
            (`/Game/Game/Interface/BPI_Character.ToggleAttacking` false _lolcked_enemy)
            (`KismetSystemLibrary.Delay` (`KismetMathLibrary.RandomFloatInRange` 3.0 7.0))))
        (if (`self.in Attack mode`)
          (goto _label_7))))
    (else
      (`/Game/Game/Interface/BPI_Character.ToggleAttacking` false)
      (`/Game/Game/Interface/BPI_Character.Lockon` null))))

(event `/Game/Game/Interface/BPI_Damageable.OnWeaponHit Gobin`
  (params (`Source Weapon Hit` :type "Actor Object Reference") (`HIt Location` :type "Vector Structure") (KnockBack :type Boolean))
  (bind _returnvalue (`self.K2_GetActorLocation`))
  (bind _returnvalue_2 (`self.K2_GetActorLocation` `Source Weapon Hit`))
  (bind (_returnvalue_roll _returnvalue_pitch _returnvalue_yaw) (`KismetMathLibrary.BreakRotator` (`KismetMathLibrary.FindLookAtRotation` _returnvalue _returnvalue_2)))
  (bind _yes_no (message `/Game/Game/Interface/BPI_Character.isEnemy` `Source Weapon Hit` (`self.team`)))
  (if _yes_no
    (if (`self.dodging`)
      _
      (elif KnockBack
        (`self.PlayAnimMontage` "/Game/Game/Mesh/Monster/Ice_Spirit/Ice_Spirit_Animation/Ice_Spirit_Konck_Back_Montage.Ice_Spirit_Konck_Back_Montage")
        (`KismetSystemLibrary.MoveComponentTo` (`self.CapsuleComponent`) (+ _returnvalue_2 (* (`KismetMathLibrary.Normal` (- _returnvalue _returnvalue_2)) 300.0)) (`KismetMathLibrary.MakeRotator` 0.0 0.0 _returnvalue_yaw) false false 0.1)
        (bind _currenthammer (message `/Game/Game/Interface/BPI_Character.GetHammer` `Source Weapon Hit`))
        (bind _returnvalue_3 (`GameplayStatics.SpawnEmitterAttached` "/Game/Game/particle/P_Fire_Burning.P_Fire_Burning" (`self.CapsuleComponent`)))
        (set `ParticleSystemComponent.InstanceParameters` (`|MakeArray` (make `ParticleSysParam` "VertSurfaceActor" "PSPT_Actor" 0.0 0.0 (0.0 0.0 0.0) (0.0 0.0 0.0) (struct) self)) _returnvalue_3)
        (bind _output_get (set `self.All Sockets` (`SceneComponent.GetAllSocketNames` (`self.Mesh`))))
        (bind (_location _head_shot_ _bone_name) (`self.Get Closest Socet` (`self.K2_GetActorLocation`) _output_get))
        (`GameplayStatics.SpawnDecalAttached` "/Game/Game/Meterial/IceLake.IceLake" (10.0 10.0 10.0) (`self.Mesh`) _bone_name _location)
        (`KismetArrayLibrary.Array_RemoveItem` (`self.All Sockets`) _bone_name)
        (bind _dmg (message `/Game/Game/Interface/BPI_weapon.GetDamge` _currenthammer))
        (`self.UpdateHealth` _dmg `Source Weapon Hit`
          (:`False`
            (`KismetSystemLibrary.Delay` 0.5)))
        (elif (`self.Blocking`)
          (`self.PlayAnimMontage` "/Game/Game/Mesh/Monster/Monster_Goblin_Mesh/Animations/Standing_Block_React_Large_mixamo_com_Montage.Standing_Block_React_Large_mixamo_com_Montage")
          (`|ExecutionSequence`
            (:`then_0`
              (`KismetSystemLibrary.Delay` 0.2)
              (if (`self.Blocking`)
                (`self.PlayAnimMontage` "/Game/Game/Mesh/Monster/Monster_Goblin_Mesh/Animations/Standing_Block_Idle_mixamo_com_Montage.Standing_Block_Idle_mixamo_com_Montage")))
            (:`then_1`
              (`CharacterMovementComponent.AddImpulse` (`self.CharacterMovement`) (* (`self.GetActorForwardVector` self) -500.0) true :!label _label_8)
              (`KismetSystemLibrary.Delay` 0.3)
              (`self.RotateToActor` `Source Weapon Hit`)))
          (else
            (`self.PlayAnimMontage` "/Game/Game/Mesh/Monster/Monster_Goblin_Mesh/AnimMontage/Goblin_HitReaction_Montage.Goblin_HitReaction_Montage")
            (bind (_currenthammer_2 _hammer) (message `/Game/Game/Interface/BPI_Character.GetHammer` `Source Weapon Hit`))
            (if _hammer
              (bind _dmg_2 (message `/Game/Game/Interface/BPI_weapon.GetDamge` _currenthammer_2))
              (`self.UpdateHealth` _dmg_2 `Source Weapon Hit`
                (:`True`
                  _))
              (else
                (bind _currentsword (message `/Game/Game/Interface/BPI_Character.GetSword` `Source Weapon Hit`))
                (bind _dmg_3 (message `/Game/Game/Interface/BPI_weapon.GetDamge` _currentsword))
                (`self.UpdateHealth` _dmg_3 `Source Weapon Hit`
                  (:`True`
                    _))))
            (`GameplayStatics.PlaySoundAtLocation` null (`self.K2_GetActorLocation`) (struct) 1.0 1.0 0.0 null null null)
            (goto _label_8)))))))

(fn `Get Closest Enemy`
  (returns (closestEnemy :type "Actor Object Reference"))
  (bind _returnvalue (`self.K2_GetActorLocation`))
  (set `self.closestEnemy` null)
  (bind _outhits (`KismetSystemLibrary.SphereTraceMultiForObjects` _returnvalue _returnvalue 1000.0 (`|MakeArray` "ObjectTypeQuery3" :!type "EObjectTypeQuery Enum")))
  (for _array_element _outhits
    (bind _yes_no (message `/Game/Game/Interface/BPI_Character.isEnemy` (`.HitActor` (`GameplayStatics.BreakHitResult` _array_element)) (`self.team`)))
    (if _yes_no
      (`/Engine/EditorBlueprintResources/StandardMacros.IsValid` (`self.closestEnemy`)
        (:`Is Valid`
          (if (not (< (`self.GetDistanceTo` (`self.closestEnemy`) self) (`self.GetDistanceTo` (`.HitActor` (`GameplayStatics.BreakHitResult` _array_element)) self)))
            (set `self.closestEnemy` (`.HitActor` (`GameplayStatics.BreakHitResult` _array_element)) :!label _label)))
        (:`Is Not Valid`
          (goto _label)))))
  (return (`self.closestEnemy`)))

(fn `Get Closest Socet`
  (params (`Hit Location` :type "Vector Structure") (SocketArray :type "Array of Name"))
  (returns (Location :type "Vector Structure") (`Head Shot?` :type Boolean) (`Bone Name` :type Name))
  (bind _mesh (`self.Mesh`))
  (bind _closest_socket (`self.Closest Socket`))
  (bind _returnvalue (`KismetMathLibrary.VSize` (- (`SceneComponent.GetSocketLocation` _mesh "None") `Hit Location`)))
  (for _array_element SocketArray
    (if (< _returnvalue (`self.Distance`))
      (set `self.Closest Socket` _array_element)
      (set `self.Distance` _returnvalue)))
  (return (`SceneComponent.GetSocketLocation` _mesh _closest_socket) (== _closest_socket "Head") _closest_socket))

(fn `GetHammer`
  (returns (CurrentHammer :type "Actor Object Reference") (Hammer :type Boolean))
  (return null false))

(fn `GetSword`
  (returns (CurrentSword :type "Actor Object Reference") (Sword :type Boolean))
  (return null false))

(fn `GetTeam`
  (returns (`team number` :type Integer))
  (return (`self.Team`)))

(fn `Is Dead`
  (returns (Dead :type Boolean))
  (return (<= (`self.Health`) 0.0)))

(fn `isBlockingOrDodging`
  (returns (blocking :type Boolean) (dodging :type Boolean))
  (return (`self.Blocking`) (`self.dodging`)))

(fn `isEnemy`
  (params (`team number` :type Integer))
  (returns (`yes/no` :type Boolean))
  (return (and (!= `team number` (`self.Team`)) (not (`self.Is Dead`)))))

(fn `isunderAttack`
  (params (`Attack Duration` :type "Float (double-precision)"))
  (returns (`under Attack` :type Boolean))
  (if (`self.under Attack`)
    (return true)
    (else
      (`self.SetunderAttack` `Attack Duration`)
      (return false))))

(fn `ON_Reaction`
  (returns (Reaction :type Boolean))
  (bind _reaction (message `/Game/Game/Interface/BPI_Ai.OnReaction_AI` (`self.GetController`)))
  (return _reaction))

(fn `UserConstructionScript`)