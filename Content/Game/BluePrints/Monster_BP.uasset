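; Goblin melee enemy that chases and attacks the player, then drops apple pickups on death.
; Tick updates flat distance and direction to the player, driving a distance-based idle/follow state machine that starts looping slash montages up close.
; Animation-end and collision-window events control attack repeats and the damaging capsule.
; Damage triggers a material flash, hit reaction, impulse and brief invulnerability through IsHit, or death and delayed removal.
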(event `self.ReceiveTick`
  (params (DeltaSeconds :type "Float (single-precision)"))
  ;[1 1 1] Monster Logic
  (`self.SaveDisAndDir`)
  (set `self.IsDeathPlayerChar` false)
  (if (`self.IsDeathPlayerChar`)
    (set `self.CurState` "NewEnumerator3"))
  (switch `/Game/Game/Maps/Level1Contents/Enums/MonsterState` (`self.CurState`)
    (:`NewEnumerator0`
      (if (<= (`self.DistancePlayerChar`) 1000.0)
        (set `self.CurState` "NewEnumerator1")))
    (:`NewEnumerator1`
      (if (<= (`self.DistancePlayerChar`) 150.0)
        (set `self.CurState` "NewEnumerator2")
        (`self.PlayAnimMontage` "/Game/Game/Mesh/Monster/Monster_Goblin_Mesh/AnimMontage/Golblin_slash_Montage.Golblin_slash_Montage")
        (set `self.IsAttacking` true)
        (elif (>= (`self.DistancePlayerChar`) 1500.0)
          (set `self.CurState` "NewEnumerator0")
          (else
            (`self.AddMovementInput` (`self.DirToPlayerChar`))))))))

(event `self.ReceiveAnyDamage`
  (params (Damage :type "Float (single-precision)") (DamageType :type "DamageType Object Reference") (InstigatedBy :type "Controller Object Reference") (DamageCauser :type "Actor Object Reference"))
  ;[1 1 1] Any Damage_Event
  (if (`self.IsHit`)
    (bind _output_get (set `self.HP` (- (`self.HP`) Damage)))
    (`self.ChangeDamageColor`)
    (if (<= _output_get 0.0)
      (`self.PlayAnimMontage` "/Game/Game/Mesh/Monster/Monster_Goblin_Mesh/AnimMontage/Goblin_death_montage.Goblin_death_montage")
      (set `self.CurState` "NewEnumerator4")
      (`PrimitiveComponent.SetCollisionEnabled` (`self.CapsuleComponent`) "NoCollision")
      (`PrimitiveComponent.SetCollisionEnabled` (`self.Capsule`) "NoCollision")
      (`KismetSystemLibrary.Delay` 5.0)
      (`self.K2_DestroyActor`)
      (`|SpawnActorFromClass` "/Game/Game/BluePrints/PlayerCharacter/InventorySystem/Blueprints/ItemClasses/BP_PickupActor.BP_PickupActor_C" (`KismetMathLibrary.MakeTransform` (`KismetMathLibrary.MakeVector` (.x (.location (`self.GetTransform`))) (.y (.location (`self.GetTransform`))) (- (.z (.location (`self.GetTransform`))) 150.0)) (.rotation (`self.GetTransform`)) (.scale (`self.GetTransform`))) "AdjustIfPossibleButAlwaysSpawn" "OverrideRootScale" null "/Game/Game/BluePrints/PlayerCharacter/InventorySystem/Blueprints/ItemClasses/Item_Food_Apple.Item_Food_Apple_C" (`KismetMathLibrary.RandomIntegerInRange` 1 5) null)
      (else
        (bind _returnvalue (`self.PlayAnimMontage` "/Game/Game/Mesh/Monster/Monster_Goblin_Mesh/AnimMontage/Goblin_HitReaction_Montage.Goblin_HitReaction_Montage" 1.5))
        (`CharacterMovementComponent.AddImpulse` (`self.CharacterMovement`) (- (`self.GetActorForwardVector` self) 1000.0) true)
        (`KismetSystemLibrary.Delay` _returnvalue)
        (set `self.CurState` "NewEnumerator1")
        (set `self.IsHit` false)
        (`KismetSystemLibrary.Delay` 1.0)
        (set `self.IsHit` true)))))

(event `self.Capsule.OnComponentBeginOverlap`
  (params (OverlappedComponent :type "PrimitiveComponent Object Reference") (OtherActor :type "Actor Object Reference") (OtherComp :type "PrimitiveComponent Object Reference") (OtherBodyIndex :type Integer) (bFromSweep :type Boolean) (SweepResult :type "HitResult Structure (by ref)"))
  ;[1 1 1] ApplyDamage
  (if (!= OtherActor self)
    (if (!= (`|GetArrayItem` (`self.Tags`)) (`|GetArrayItem` (`Actor.Tags` OtherActor)))
      (if (== (`|GetArrayItem` (`ActorComponent.ComponentTags` OtherComp)) "Character")
        (`GameplayStatics.ApplyDamage` OtherActor (`self.Atk`) null self)))))

(event `OnAnimEnd_Attack`
  ;[1 1 1] OnAnimEndAttack_Event
  (set `self.IsAttacking` false)
  (if (`self.IsDeathPlayerChar`)
    (set `self.CurState` "NewEnumerator3")
    (elif (>= (`self.DistancePlayerChar`) 180.0)
      (set `self.CurState` "NewEnumerator1")
      (else
        (`self.K2_SetActorRotation` (`KismetMathLibrary.Conv_VectorToRotator` (`self.DirToPlayerChar`)))
        (`self.PlayAnimMontage` "/Game/Game/Mesh/Monster/Monster_Goblin_Mesh/AnimMontage/Golblin_slash_Montage.Golblin_slash_Montage")
        (set `self.IsAttacking` true)))))

(event `OnColStart_Attack`
  ;[1 1 1] AxeCollision_processing
  (`PrimitiveComponent.SetCollisionEnabled` (`self.Capsule`) "QueryAndPhysics"))

(event `OnColEnd_Attack`
  ;[1 1 1] AxeCollision_processing
  (`PrimitiveComponent.SetCollisionEnabled` (`self.Capsule`) "NoCollision"))

(event `SaveDisAndDir`
  (bind _returnvalue (`GameplayStatics.GetPlayerCharacter` 0))
  (bind _returnvalue_2 (`KismetMathLibrary.MakeVector` (.x (- (`self.K2_GetActorLocation` _returnvalue) (`self.K2_GetActorLocation`))) (.y (- (`self.K2_GetActorLocation` _returnvalue) (`self.K2_GetActorLocation`)))))
  ;[1 1 1] SaveDisAndDir_Event
  (if (`self.IsHit`)
    (bind _asthird_person_character (cast `/Game/Game/BluePrints/PlayerCharacter/ThirdPersonCharacter` _returnvalue))
    (set `self.IsDeathPlayerChar` (`/Game/Game/BluePrints/PlayerCharacter/ThirdPersonCharacter.IsDeath` _asthird_person_character))
    (set `self.DistancePlayerChar` (`KismetMathLibrary.VSize` _returnvalue_2))
    (set `self.DirToPlayerChar` (`KismetMathLibrary.Vector_NormalUnsafe` _returnvalue_2))))

(event `ChangeDamageColor`
  ;[1 1 1] ChangeDamageColor_Event
  (`PrimitiveComponent.SetMaterial` (`self.Mesh`) 0 "/Game/Game/Mesh/Monster/Monster_Goblin_Mesh/phong1_Inst.phong1_Inst")
  (`KismetSystemLibrary.Delay` 0.2)
  (`PrimitiveComponent.SetMaterial` (`self.Mesh`) 0 "/Game/Game/Mesh/Monster/Monster_Goblin_Mesh/phong1.phong1"))

(fn `UserConstructionScript`)