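; BP_Snow_Plane is a snow surface actor that records left and right foot marks into the RT_Snow_Plane render target.
; On BeginPlay it creates a dynamic brush material from M_Foot_Brush_Inst and clears the render target to black.
; Its Draw event takes two 2D positions, writes each into the brush's right or left vector parameter, and draws the material to the render target after each update.
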(event `self.ReceiveBeginPlay`
  (bind _returnvalue (`KismetMaterialLibrary.CreateDynamicMaterialInstance` "/Game/Game/RenderTarget/M_Foot_Brush_Inst.M_Foot_Brush_Inst"))
  (set `self.Brush_reff` _returnvalue)
  (`KismetRenderingLibrary.ClearRenderTarget2D` "/Game/Game/RenderTarget/RT_Snow_Plane.RT_Snow_Plane"))

(event `Draw`
  (params (Right :type "Vector2D Structure") (LEft :type "Vector2D Structure"))
  (bind _brush_reff (`self.Brush_reff`))
  (bind _brush_reff_2 (`self.Brush_reff`))
  (`|ExecutionSequence`
    (:`then_0`
      (`MaterialInstanceDynamic.SetVectorParameterValue` _brush_reff "right" (`KismetMathLibrary.Conv_VectorToLinearColor` (`KismetMathLibrary.Conv_Vector2DToVector` Right)))
      (`KismetRenderingLibrary.DrawMaterialToRenderTarget` "/Game/Game/RenderTarget/RT_Snow_Plane.RT_Snow_Plane" _brush_reff_2))
    (:`then_1`
      (`MaterialInstanceDynamic.SetVectorParameterValue` _brush_reff "left" (`KismetMathLibrary.Conv_VectorToLinearColor` (`KismetMathLibrary.Conv_Vector2DToVector` LEft)))
      (`KismetRenderingLibrary.DrawMaterialToRenderTarget` "/Game/Game/RenderTarget/RT_Snow_Plane.RT_Snow_Plane" _brush_reff_2))))

(fn `UserConstructionScript`)