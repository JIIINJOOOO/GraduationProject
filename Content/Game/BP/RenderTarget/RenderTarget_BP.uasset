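; Snow render-target actor with a SceneCapture2D whose capture area can follow the player, publishing its size and location to Snow_MPC.
; BeginPlay clears both render targets, creates a dynamic DrawToPersistent material and sets a short timer that draws it into the persistent target.
; MoveRT shifts the actor in XY to the player's position snapped to a pixel grid (ortho width / 256), then updates CaptureLocation.
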(event `self.ReceiveBeginPlay`
  (`|ExecutionSequence`
    (:`then_0`
      (`KismetMaterialLibrary.SetScalarParameterValue` "/Game/Game/BP/RenderTarget/Snow_MPC.Snow_MPC" "Size" (`SceneCaptureComponent2D.OrthoWidth` (`self.SceneCaptureComponent2D`)))
      (bind _returnvalue (`KismetMaterialLibrary.CreateDynamicMaterialInstance` "/Game/Game/BP/RenderTarget/DrawToPersistent.DrawToPersistent"))
      (set `self.DrawToMat` _returnvalue)
      (`KismetRenderingLibrary.ClearRenderTarget2D` "/Game/Game/BP/RenderTarget/RenderTarget.RenderTarget")
      (`KismetRenderingLibrary.ClearRenderTarget2D` "/Game/Game/BP/RenderTarget/RenderTargetPersistent.RenderTargetPersistent"))
    (:`then_1`
      (`KismetSystemLibrary.K2_SetTimer` null "DrawToRT" 0.01))))

(event `DrawToRT`
  (`KismetRenderingLibrary.DrawMaterialToRenderTarget` "/Game/Game/BP/RenderTarget/RenderTargetPersistent.RenderTargetPersistent" (`self.DrawToMat`)))

(event `MoveRT`
  (bind (_returnvalue_x _returnvalue_y) (`KismetMathLibrary.BreakVector` (`self.K2_GetActorLocation` (`GameplayStatics.GetPlayerCharacter` 0))))
  (bind (_returnvalue_x_2 _returnvalue_y_2) (`KismetMathLibrary.BreakVector` (- (`self.SnapPixeIToGrid` _returnvalue_x _returnvalue_y (* (`SceneCaptureComponent2D.OrthoWidth` (`self.SceneCaptureComponent2D`)) (/ 1.0 256.0))) (`self.K2_GetActorLocation`))))
  (bind _output_get (set `self.MoveOffset` (`KismetMathLibrary.MakeVector2D` _returnvalue_x_2 _returnvalue_y_2)))
  (`self.K2_AddActorWorldOffset` (`KismetMathLibrary.MakeVector` (`KismetMathLibrary.BreakVector2D` _output_get) (`.Y` (`KismetMathLibrary.BreakVector2D` _output_get))))
  (`KismetMaterialLibrary.SetVectorParameterValue` "/Game/Game/BP/RenderTarget/Snow_MPC.Snow_MPC" "CaptureLocation" (`KismetMathLibrary.Conv_VectorToLinearColor` (`self.K2_GetActorLocation`))))

(fn `UserConstructionScript`)